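; BP_Hexgrid is an actor that generates a hex-style grid of static mesh tiles, sized by grid and spacing variables.
; The Construction Script adds one mesh per cell, shifting odd X columns along Y by an offset, and stores grid coordinates in TilesArr.
; BeginPlay draws each tile's index as debug text, using world positions that add the offset to every Y step, so labels differ from the mesh layout.
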(event `self.ReceiveBeginPlay`
  (for (_array_element _array_index) (`self.TilesArr`)
    (`KismetSystemLibrary.DrawDebugString` (`KismetMathLibrary.MakeVector` (* (`self.SpacingX`) (.x _array_element)) (* (+ (`self.SpacingY`) (`self.Offset`)) (.y _array_element)) 200.0) (`KismetStringLibrary.Conv_IntToString` _array_index) null (struct :`R` 1.0 :`A` 1.0) 100.0)))

(fn `UserConstructionScript`
  (for _index (range (+ (`self.GridX`) 1))
    (for _index_2 (range (+ (`self.GridY`) 1))
      (`KismetArrayLibrary.Array_Add` (`self.TilesArr`) (`KismetMathLibrary.MakeVector` (`KismetMathLibrary.Conv_IntToDouble` _index) (`KismetMathLibrary.Conv_IntToDouble` _index_2)))
      (bind _returnvalue (* _index (`self.SpacingX`)))
      (bind _returnvalue_2 (* _index_2 (`self.SpacingY`)))
      (`AddComponent|NODE_AddStaticMeshComponent-0` :`RelativeTransform` (`KismetMathLibrary.MakeTransform` (`KismetMathLibrary.SelectVector` (`KismetMathLibrary.MakeVector` _returnvalue _returnvalue_2) (`KismetMathLibrary.MakeVector` _returnvalue (+ (`self.Offset`) _returnvalue_2)) (== (mod _index 2) 0)))))))
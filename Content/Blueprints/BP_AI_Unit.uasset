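; Selectable RTS skirmish unit that moves under AI control, supporting selection highlighting, a portrait UI widget and camera follow for friendly units.
; BeginPlay picks a random patrol point; Tick turns and moves the unit toward its current target vector.
; Pawn sensing retargets onto seen units, still cast to a deprecated class, and adjusts engage distance.
; Construction spawns child actors at hardpoints, and Tick passes targeting data to child turrets.
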(event `/Game/Blueprints/Interfaces/Skirmish_Interface.HighlightUnit`
  ;[1 1 1] Unit Selection
  (`PrimitiveComponent.SetMaterial` (`self.Selection`) 0 "/Engine/ArtTools/RenderToTexture/Materials/Debug/M_Emissive_Color_0-0-127.M_Emissive_Color_0-0-127"))

(event `/Game/Blueprints/Interfaces/Skirmish_Interface.UnHighlightUnit`
  ;[1 1 1] Unit Selection
  (`PrimitiveComponent.SetMaterial` (`self.Selection`) 0 "/Game/AdvancedTurnBasedTileToolkit/Core/GridUI/M_EmissiveMask.M_EmissiveMask"))

(event `/Game/Blueprints/Interfaces/Skirmish_Interface.SelectUnit`
  ;[1 1 1] Unit Selection
  (`SceneComponent.SetVisibility` (`self.Selection`) true false)
  (set `self.IsSelected` true)
  (message `/Game/Blueprints/Interfaces/Skirmish_Interface.AddSelectedUnitToUI` (`GameplayStatics.GetPlayerController` 0) (`self.SelectedUnitWidget`)))

(event `/Game/Blueprints/Interfaces/Skirmish_Interface.DeselectUnit`
  ;[1 1 1] Unit Selection
  (`SceneComponent.SetVisibility` (`self.Selection`) false false)
  (set `self.IsSelected` false)
  (`Widget.RemoveFromParent` (`self.SelectedUnitWidget`)))

(event `/Game/Blueprints/Interfaces/Skirmish_Interface.UnitMoveCommand`
  (params (Location :type "Vector Structure"))
  (set `self.TargetVector` Location))

(event `self.ReceiveBeginPlay`
  (`self.SetPatrol`)
  (if (`self.ActorHasTag` "Friendly")
    (bind _bp_openrtscamera (`/Game/Plugins/OpenRTSCamera/Content/BPFL_RTSCameraSystem.Get OpenRTS Camera`))
    (`RTSCamera.FollowTarget` (`/OpenRTSCamera/BP_RTSCamera.RTSCamera` _bp_openrtscamera) self)
    (bind _returnvalue (`|CreateWidget` "/Game/Blueprints/UI/WB_Skirmish_Selected_Unit.WB_Skirmish_Selected_Unit_C"))
    (set `/Game/Blueprints/UI/WB_Skirmish_Selected_Unit.UnitReference` self _returnvalue)
    (`Image.SetBrushFromTexture` (`/Game/Blueprints/UI/WB_Skirmish_Selected_Unit.UnitImage` _returnvalue) (`self.UNIT_Portrait`) false)
    (set `self.SelectedUnitWidget` _returnvalue)))

(event `self.ReceiveTick`
  (params (DeltaSeconds :type "Float (single-precision)"))
  ;[1 1 1] AI
  (`|ExecutionSequence`
    (:`then_0`
      (`self.newRotateTo` DeltaSeconds))
    (:`then_1`
      (`AITask_MoveTo.AIMoveTo` (`AIBlueprintHelperLibrary.GetAIController` self) (`self.TargetVector`) null (`self.EngageDistance`) "Enable" "Disable" true true (`self.CanMove`) "Disable"
        (:`OnMoveFinished`
          (`self.TargetUnit`
            (:`then`)
            (:`else`
              (`KismetSystemLibrary.Delay` 2.0))))))
    (:`then_2`
      (`self.TargetUnit`
        (:`then`
          (if (`PawnSensingComponent.bSeePawns` (`self.PawnSensing`))
            (set `self.TargetVector` (`self.K2_GetActorLocation` (`self.TargetUnit`)))
            (set `self.CanSeeEnemy` true)
            (set `self.EngageDistance` (/ (`self.SensorRange`) 2.0))
            (else
              (set `self.CanSeeEnemy` false)
              (set `self.EngageDistance` 10.0)
              (set `self.TargetUnit` null))))
        (:`else`)))
    (:`then_3`
      (bind _filteredarray (`KismetArrayLibrary.FilterArray` (`self.GetAllChildActors` true) "/Game/Blueprints/Components/BP_Turret_Base.BP_Turret_Base_C"))
      (for _array_element _filteredarray
        (bind _asbp_turret_base (cast `/Game/Blueprints/Components/BP_Turret_Base` _array_element))
        (set `/Game/Blueprints/Components/BP_Turret_Base.TargetVector` (`self.TargetVector`) _asbp_turret_base)
        (set `/Game/Blueprints/Components/BP_Turret_Base.CanSeeEnemy` (`self.CanSeeEnemy`) _asbp_turret_base)
        (set `/Game/Blueprints/Components/BP_Turret_Base.EngageDistance` (`self.EngageDistance`) _asbp_turret_base)))))

(event `self.PawnSensing.OnSeePawn`
  (params (Pawn :type "Pawn Object Reference"))
  ;[1 1 1] REFACTOR - Visibility for enemy units
  (bind _asbp_skirmish_unit (cast `/Game/Blueprints/Units/DEPRECATED_BP_Skirmish_Unit` Pawn))
  (set `self.TargetUnit` _asbp_skirmish_unit)
  (bind _returnvalue (`self.K2_GetActorLocation` _asbp_skirmish_unit))
  (set `self.TargetVector` (`KismetMathLibrary.MakeVector` (.x _returnvalue) (.y _returnvalue)))
  (if (< (`KismetMathLibrary.Vector_Distance2D` (`self.K2_GetActorLocation`) _returnvalue) (`self.SensorRange`))
    (set `self.CanSeeEnemy` true)
    (else
      (set `self.CanSeeEnemy` false))))

(fn `GrabSelectedUnits`
  (returns (`Selected Units` :type "Array of Actor Object Reference"))
  (return))

(fn `newRotateTo`
  (params (DeltaTime :type "Float (single-precision)"))
  (bind (_returnvalue_roll _returnvalue_pitch _returnvalue_yaw) (`KismetMathLibrary.BreakRotator` (`KismetMathLibrary.RInterpTo` (`self.K2_GetActorRotation`) (`KismetMathLibrary.FindLookAtRotation` (`self.K2_GetActorLocation`) (`self.TargetVector`)) DeltaTime 0.7)))
  (if (not (`self.IsWithinDistance`))
    (`self.K2_SetActorRotation` (`KismetMathLibrary.MakeRotator` _returnvalue_roll 0.0 _returnvalue_yaw) true)))

(fn `rotateToTarget`
  (params (TargetLocation :type "Vector Structure")))

(fn `SetPatrol`
  (if (`self.CanSeeEnemy`)
    _
    (else
      _))
  (bind _output_get (set `self.TargetVector` (`KismetMathLibrary.MakeVector` (.x (`NavigationSystemV1.K2_GetRandomReachablePointInRadius` (`self.K2_GetActorLocation`) (`self.PatrolRadius`) null null)) (.y (`NavigationSystemV1.K2_GetRandomReachablePointInRadius` (`self.K2_GetActorLocation`) (`self.PatrolRadius`) null null)) (`self.zIndex`))))
  (`KismetSystemLibrary.PrintString` (`KismetStringLibrary.Conv_VectorToString` _output_get))
  (`KismetSystemLibrary.DrawDebugSphere` _output_get 100.0 12 (struct :`R` 0.681644 :`G` 0.003043 :`B` 1.0 :`A` 1.0) 5.0 2.0)
  (return))

(fn `UserConstructionScript`
  (bind (_returnvalue_x _returnvalue_y) (`KismetMathLibrary.BreakVector` (`self.K2_GetActorLocation`)))
  (`self.K2_SetActorRelativeLocation` (`KismetMathLibrary.MakeVector` _returnvalue_x _returnvalue_y (`self.zIndex`)) false true)
  ;[1 1 1] Construct Hardpoint Instances
  (for _array_element (`SceneComponent.GetChildrenComponents` (`self.Hardpoints`) false)
    (`AddComponent|NODE_AddChildActorComponent-3` :`RelativeTransform` (`KismetMathLibrary.MakeTransform` (`SceneComponent.RelativeLocation` _array_element)))))
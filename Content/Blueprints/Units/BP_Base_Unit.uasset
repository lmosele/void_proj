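; Base RTS skirmish unit pawn with selection highlighting, selection UI widget, random patrolling and enemy pursuit.
; On BeginPlay it spawns and attaches a UNITClass puppet actor, whose stats set movement, turning, sensor and patrol values.
; Tick turns and moves it toward TargetVector, set by commands, patrol or PawnSensing, and relays targeting to child turrets.
; Turret spawning and debug visualisers are unwired; sensing still casts to a deprecated unit class.
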(event `/Game/Blueprints/Interfaces/Skirmish_Interface.HighlightUnit`
  ;[1 1 1] Unit Selection
  (`PrimitiveComponent.SetMaterial` (`self.Selection`) 0 "/Engine/ArtTools/RenderToTexture/Materials/Debug/M_Emissive_Color_0-0-127.M_Emissive_Color_0-0-127"))

(event `/Game/Blueprints/Interfaces/Skirmish_Interface.UnHighlightUnit`
  ;[1 1 1] Unit Selection
  (`PrimitiveComponent.SetMaterial` (`self.Selection`) 0 "/Game/AdvancedTurnBasedTileToolkit/Core/GridUI/M_EmissiveMask.M_EmissiveMask"))

(event `/Game/Blueprints/Interfaces/Skirmish_Interface.SelectUnit`
  ;[1 1 1] Unit Selection
  (`SceneComponent.SetVisibility` (`self.Selection`) true false)
  (set `self.IsSelected` true)
  (message `/Game/Blueprints/Interfaces/Skirmish_Interface.AddSelectedUnitToUI` (`GameplayStatics.GetPlayerController` 0) (`self.SelectedUnitWidget`)))

(event `/Game/Blueprints/Interfaces/Skirmish_Interface.DeselectUnit`
  ;[1 1 1] Unit Selection
  (`SceneComponent.SetVisibility` (`self.Selection`) false false)
  (set `self.IsSelected` false)
  (`Widget.RemoveFromParent` (`self.SelectedUnitWidget`)))

(event `/Game/Blueprints/Interfaces/Skirmish_Interface.UnitMoveCommand`
  (params (Location :type "Vector Structure"))
  (set `self.TargetVector` Location))

(event `self.ReceiveBeginPlay`
  (bind (_unit_stats_unit_health _unit_stats_unit_mesh _unit_stats_unit_speed _unit_stats_unit_turn_rate _unit_stats_unit_accel _unit_stats_unit_faction _unit_stats_unit_patrol_radius _unit_stats_unit_sensor_range _unit_stats_unit_z_location _unit_stats_unit_engage_distance _unit_stats_unit_mesh_scale _unit_stats_unit_mesh_rotation _unit_stats_unit_portrait) (break `/Game/Blueprints/Units/UnitStatsStruct` (`/Game/Blueprints/Units/BP_Unit_Puppet_Default.UNIT_Stats` (`self.UNIT_Puppet_Ref`))))
  (`self.SetPuppetAttributes`)
  (`|ExecutionSequence`
    (:`then_0`
      (bind _returnvalue (`|CreateWidget` "/Game/Blueprints/UI/WB_Skirmish_Selected_Unit.WB_Skirmish_Selected_Unit_C"))
      (set `/Game/Blueprints/UI/WB_Skirmish_Selected_Unit.UnitReference` self _returnvalue)
      (`Image.SetBrushFromTexture` (`/Game/Blueprints/UI/WB_Skirmish_Selected_Unit.UnitImage` _returnvalue) _unit_stats_unit_portrait false)
      (set `self.SelectedUnitWidget` _returnvalue))
    (:`then_1`
      (`self.SetPatrol`))
    (:`then_2`
      (if (`self.IsSelected`)
        (bind _bp_openrtscamera (`/Game/Plugins/OpenRTSCamera/Content/BPFL_RTSCameraSystem.Get OpenRTS Camera`))
        (`RTSCamera.FollowTarget` (`/OpenRTSCamera/BP_RTSCamera.RTSCamera` _bp_openrtscamera) self)))))

(event `self.ReceiveTick`
  (params (DeltaSeconds :type "Float (single-precision)"))
  ;[1 1 1] AI
  (`|ExecutionSequence`
    (:`then_0`
      (`self.RotateToTarget` DeltaSeconds))
    (:`then_1`
      (`AITask_MoveTo.AIMoveTo` (`AIBlueprintHelperLibrary.GetAIController` self) (`self.TargetVector`) null (`self.EngageDistance`) "Enable" "Disable" true true (`self.CanMove`) "Disable"
        (:`OnMoveFinished`
          (`KismetSystemLibrary.Delay` 2.0)
          (`self.SetPatrol`))))
    (:`then_2`
      (`self.TargetUnit`
        (:`then`
          (if (`PawnSensingComponent.bSeePawns` (`self.PawnSensing`))
            (set `self.TargetVector` (`self.K2_GetActorLocation` (`self.TargetUnit`)))
            (set `self.CanSeeEnemy` true)
            (set `self.EngageDistance` (/ (`self.SensorRange`) 2.0))
            (else
              (set `self.CanSeeEnemy` false)
              (set `self.EngageDistance` 10.0)
              (set `self.TargetUnit` null))))
        (:`else`)))
    (:`then_3`
      (bind _filteredarray (`KismetArrayLibrary.FilterArray` (`self.GetAllChildActors` true) "/Game/Blueprints/Components/BP_Turret_Base.BP_Turret_Base_C"))
      (for _array_element _filteredarray
        (bind _asbp_turret_base (cast `/Game/Blueprints/Components/BP_Turret_Base` _array_element))
        (set `/Game/Blueprints/Components/BP_Turret_Base.TargetVector` (`self.TargetVector`) _asbp_turret_base)
        (set `/Game/Blueprints/Components/BP_Turret_Base.CanSeeEnemy` (`self.CanSeeEnemy`) _asbp_turret_base)
        (set `/Game/Blueprints/Components/BP_Turret_Base.EngageDistance` (`self.EngageDistance`) _asbp_turret_base)))))

(event `self.PawnSensing.OnSeePawn`
  (params (Pawn :type "Pawn Object Reference"))
  ;[1 1 1] REFACTOR - Visibility for enemy units
  (bind _asdeprecated_bp_skirmish_unit (cast `/Game/Blueprints/Units/DEPRECATED_BP_Skirmish_Unit` Pawn))
  (set `self.TargetUnit` _asdeprecated_bp_skirmish_unit)
  (bind _returnvalue (`self.K2_GetActorLocation` _asdeprecated_bp_skirmish_unit))
  (set `self.TargetVector` (`KismetMathLibrary.MakeVector` (.x _returnvalue) (.y _returnvalue)))
  (if (< (`KismetMathLibrary.Vector_Distance2D` (`self.K2_GetActorLocation`) _returnvalue) (`self.SensorRange`))
    (set `self.CanSeeEnemy` true)
    (else
      (set `self.CanSeeEnemy` false))))

(fn `GrabSelectedUnits`
  (returns (`Selected Units` :type "Array of Actor Object Reference"))
  (return))

(fn `RotateToTarget`
  (params (DeltaTime :type "Float (single-precision)"))
  (bind (_returnvalue_roll _returnvalue_pitch _returnvalue_yaw) (`KismetMathLibrary.BreakRotator` (`KismetMathLibrary.RInterpTo` (`self.K2_GetActorRotation`) (`KismetMathLibrary.FindLookAtRotation` (`self.K2_GetActorLocation`) (`self.TargetVector`)) DeltaTime (`self.Turnspeed`))))
  (if (not (`self.IsWithinDistance`))
    (`self.K2_SetActorRotation` (`KismetMathLibrary.MakeRotator` _returnvalue_roll 0.0 _returnvalue_yaw) true)))

(fn `SetPatrol`
  (if (`self.CanSeeEnemy`)
    _
    (else
      _))
  (bind _output_get (set `self.TargetVector` (`KismetMathLibrary.MakeVector` (.x (`NavigationSystemV1.K2_GetRandomReachablePointInRadius` (`self.K2_GetActorLocation`) (`self.PatrolRadius`) null null)) (.y (`NavigationSystemV1.K2_GetRandomReachablePointInRadius` (`self.K2_GetActorLocation`) (`self.PatrolRadius`) null null)) (`self.zIndex`))))
  (`KismetSystemLibrary.PrintString` (`KismetStringLibrary.Conv_VectorToString` _output_get))
  (`KismetSystemLibrary.DrawDebugSphere` _output_get 100.0 12 (struct :`R` 0.681644 :`G` 0.003043 :`B` 1.0 :`A` 1.0) 5.0 2.0)
  (return))

(fn `SetPuppetAttributes`
  (bind (_unit_stats_unit_health _unit_stats_unit_mesh _unit_stats_unit_speed _unit_stats_unit_turn_rate _unit_stats_unit_accel _unit_stats_unit_faction _unit_stats_unit_patrol_radius _unit_stats_unit_sensor_range _unit_stats_unit_z_location _unit_stats_unit_engage_distance _unit_stats_unit_mesh_scale) (break `/Game/Blueprints/Units/UnitStatsStruct` (`/Game/Blueprints/Units/BP_Unit_Puppet_Default.UNIT_Stats` (`self.UNIT_Puppet_Ref`))))
  ;[1 1 1] Attach Puppet Actor to Pawn
  (if (`KismetSystemLibrary.IsValidClass` (`self.UNIT_Class`))
    (`/Engine/EditorBlueprintResources/StandardMacros.DoOnce` false
      (:`Completed`
        (bind _returnvalue (`|SpawnActorFromClass` (`self.UNIT_Class`) (`SceneComponent.GetRelativeTransform` (`self.Puppet`)) "AdjustIfPossibleButDontSpawnIfColliding" "OverrideRootScale" self self))
        (bind _output_get (set `self.UNIT_Puppet_Ref` _returnvalue))
        (`self.K2_AttachToComponent` _output_get (`self.Puppet`) "None" "KeepRelative" "KeepRelative" "KeepRelative" false)
        (`|ExecutionSequence`
          (:`then_1`
            ;[1 1 1] Set Unit Gameplay Stats
            (bind _asfloating_pawn_movement (cast `FloatingPawnMovement` (`self.MovementComponent`)))
            (set `FloatingPawnMovement.MaxSpeed` _unit_stats_unit_speed _asfloating_pawn_movement)
            (set `FloatingPawnMovement.Acceleration` _unit_stats_unit_accel _asfloating_pawn_movement)
            (set `self.Turnspeed` _unit_stats_unit_turn_rate)
            (set `self.SensorRange` _unit_stats_unit_sensor_range)
            (set `self.EngageDistance` _unit_stats_unit_engage_distance)
            (set `self.PatrolRadius` _unit_stats_unit_patrol_radius)))))))

(fn `UserConstructionScript`)
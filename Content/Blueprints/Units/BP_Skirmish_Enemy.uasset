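; BP_Skirmish_Enemy is an AI skirmish enemy that wanders around the player and chases units it sees.
; While CanSeeEnemy is false, a Tick-driven random Delay periodically sends it to a reachable point near the player, spawning an explosion effect there as the move is issued.
; PawnSensing sightings of a BP_Skirmish_Unit set CanSeeEnemy and start pursuit.
; A retriggerable delay clears the flag shortly after sightings stop.
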(event `self.ReceiveTick`
  (params (DeltaSeconds :type "Float (single-precision)"))
  (if (not (`self.CanSeeEnemy`))
    (`KismetSystemLibrary.Delay` (`KismetMathLibrary.RandomFloatInRange` 1.0 10.0))
    (bind _output_get (set `self.Random Location` (`NavigationSystemV1.K2_GetRandomReachablePointInRadius` (`self.K2_GetActorLocation` (`GameplayStatics.GetPlayerCharacter` 0)) 2000.0 null null)))
    (`|AIMoveTo` self _output_get null 5.0 true
      (:`then`
        (`GameplayStatics.SpawnEmitterAtLocation` "/Game/AdvancedTurnBasedTileToolkit/Maps/Advanced/Abilities/PS_Explosion.PS_Explosion" (`self.Random Location`))))))

(event `self.PawnSensing.OnSeePawn`
  (params (Pawn :type "Pawn Object Reference"))
  (bind _asbp_skirmish_unit (cast `/Game/Blueprints/Units/BP_Skirmish_Unit` Pawn))
  (`|ExecutionSequence`
    (:`then_0`
      (set `self.CanSeeEnemy` true)
      (`|AIMoveTo` self (0.0 0.0 0.0) _asbp_skirmish_unit))
    (:`then_1`
      (`KismetSystemLibrary.RetriggerableDelay` 0.5)
      (set `self.CanSeeEnemy` false))))

(fn `UserConstructionScript`)
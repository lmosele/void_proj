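; Parent RTS unit that navigates by AI to a target point set by random patrol, move command or pawn sensing.
; BeginPlay picks a patrol point and, for Friendly units, sets camera follow and creates a selection widget.
; Tick reissues AIMoveTo, repicking after failures; sighting a skirmish unit retargets it and flags range.
; Selection, puppet and hardpoint turret spawning, turret targeting, rotation and visibility helpers exist but are unwired.
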(event `self.ReceiveActorBeginOverlap`
  (params (OtherActor :type "Actor Object Reference"))
  (`KismetSystemLibrary.PrintString` (`KismetSystemLibrary.GetDisplayName` OtherActor)))

(event `/Game/Blueprints/Interfaces/Skirmish_Interface.HighlightUnit`
  ;[1 1 1] Unit Selection
)

(event `/Game/Blueprints/Interfaces/Skirmish_Interface.UnHighlightUnit`
  ;[1 1 1] Unit Selection
)

(event `/Game/Blueprints/Interfaces/Skirmish_Interface.SelectUnit`
  ;[1 1 1] Unit Selection
)

(event `/Game/Blueprints/Interfaces/Skirmish_Interface.DeselectUnit`
  ;[1 1 1] Unit Selection
)

(event `/Game/Blueprints/Interfaces/Skirmish_Interface.UnitMoveCommand`
  (params (Location :type "Vector Structure"))
  (set `self.TargetVector` Location))

(event `Spawn Puppet Attributes`)

(event `self.ReceiveBeginPlay`
  (`self.SetPatrol`)
  (if (`self.ActorHasTag` "Friendly")
    (bind _bp_openrtscamera (`/Game/Plugins/OpenRTSCamera/Content/BPFL_RTSCameraSystem.Get OpenRTS Camera`))
    (`RTSCamera.FollowTarget` (`/OpenRTSCamera/BP_RTSCamera.RTSCamera` _bp_openrtscamera) self)
    (bind _returnvalue (`|CreateWidget` "/Game/Blueprints/UI/WB_Skirmish_Selected_Unit.WB_Skirmish_Selected_Unit_C"))
    (set `/Game/Blueprints/UI/WB_Skirmish_Selected_Unit.UnitReference` self _returnvalue)
    (`Image.SetBrushFromTexture` (`/Game/Blueprints/UI/WB_Skirmish_Selected_Unit.UnitImage` _returnvalue) (`self.UNIT_Portrait`) false)
    (set `self.SelectedUnitWidget` _returnvalue)))

(event `self.ReceiveTick`
  (params (DeltaSeconds :type "Float (single-precision)"))
  ;[1 1 1] AI
  (`AITask_MoveTo.AIMoveTo` (`AIBlueprintHelperLibrary.GetAIController` self) (`self.TargetVector`) null (`self.EngageDistance`) "Disable" "Enable" true true false "Disable"
    (:`then`
      (`KismetSystemLibrary.PrintString` "Going"))
    (:`OnRequestFailed`
      (`KismetSystemLibrary.PrintString` "Failed")
      (`KismetSystemLibrary.Delay` 2.0)
      (`self.SetPatrol`))
    (:`OnMoveFinished`
      (`KismetSystemLibrary.PrintString` "Finished"))))

(event `self.PawnSensing.OnSeePawn`
  (params (Pawn :type "Pawn Object Reference"))
  ;[1 1 1] REFACTOR - Visibility for enemy units
  (bind _asbp_skirmish_unit (cast `/Game/Blueprints/Units/BP_Skirmish_Unit` Pawn))
  (set `self.TargetUnit` _asbp_skirmish_unit)
  (bind _returnvalue (`self.K2_GetActorLocation` _asbp_skirmish_unit))
  (set `self.TargetVector` (`KismetMathLibrary.MakeVector` (.x _returnvalue) (.y _returnvalue)))
  (if (< (`KismetMathLibrary.Vector_Distance2D` (`self.K2_GetActorLocation`) _returnvalue) (`self.SensorRange`))
    (set `self.CanSeeEnemy` true)
    (else
      (set `self.CanSeeEnemy` false))))

(fn `GrabSelectedUnits`
  (returns (`Selected Units` :type "Array of Actor Object Reference"))
  (return))

(fn `RotateToTarget`
  (params (DeltaTime :type "Float (single-precision)"))
  (locals (PreviousDirection :type "Float (single-precision)" :default 0.0) (NewLocalVar :type "Float (single-precision)" :default 0.0))
  (bind (_returnvalue_roll _returnvalue_pitch _returnvalue_yaw) (`KismetMathLibrary.BreakRotator` (`KismetMathLibrary.RInterpTo` (`self.K2_GetActorRotation`) (`KismetMathLibrary.FindLookAtRotation` (`self.K2_GetActorLocation`) (`self.TargetVector`)) DeltaTime 1.0)))
  (if (not (`self.IsWithinDistance`))
    (`self.K2_SetActorRotation` (`KismetMathLibrary.MakeRotator` 0.0 0.0 _returnvalue_yaw) true)))

(fn `SetPatrol`
  (if (`self.CanSeeEnemy`)
    _
    (else
      _))
  (bind _output_get (set `self.TargetVector` (`KismetMathLibrary.MakeVector` (.x (`NavigationSystemV1.K2_GetRandomReachablePointInRadius` (`self.K2_GetActorLocation`) (`self.PatrolRadius`) null null)) (.y (`NavigationSystemV1.K2_GetRandomReachablePointInRadius` (`self.K2_GetActorLocation`) (`self.PatrolRadius`) null null)) (`self.zIndex`))))
  (`KismetSystemLibrary.PrintString` (`KismetStringLibrary.Conv_VectorToString` _output_get))
  (`KismetSystemLibrary.DrawDebugSphere` _output_get 100.0 12 (struct :`R` 0.681644 :`G` 0.003043 :`B` 1.0 :`A` 1.0) 5.0 2.0)
  (return))

(fn `UserConstructionScript`
  (bind (_returnvalue_x _returnvalue_y) (`KismetMathLibrary.BreakVector` (`self.K2_GetActorLocation`)))
  (`self.K2_SetActorRelativeLocation` (`KismetMathLibrary.MakeVector` _returnvalue_x _returnvalue_y (`self.zIndex`)) false true))
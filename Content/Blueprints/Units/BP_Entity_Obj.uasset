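; BP_Entity_Obj is a unit entity definition holding a name, faction, health, icon, mesh and mesh transform.
; It contains only getters, which group these fields into metadata (name, faction, health, icon) and construct values (mesh, transform), plus health on its own.
; A bounds getter returns only the Max corner of the mesh's bounding box, not its full extent.
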(fn `GetConstructValues`
  (returns (Mesh :type "StaticMesh Object Reference") (MeshTransform :type "Transform Structure"))
  (return (`self.Mesh`) (`self.MeshTransform`)))

(fn `GetHealth`
  (returns (Health :type Integer))
  (return (`self.Health`)))

(fn `GetMeshBounds`
  (returns (`Return Value Max X` :type "Float (double-precision)") (`Return Value Max Y` :type "Float (double-precision)") (`Return Value Max Z` :type "Float (double-precision)"))
  (bind _returnvalue (`StaticMesh.GetBoundingBox` (`self.Mesh`)))
  (return (.x (`.Max` (break `Box` _returnvalue))) (.y (`.Max` (break `Box` _returnvalue))) (.z (`.Max` (break `Box` _returnvalue)))))

(fn `GetMetaData`
  (returns (Name :type String) (Faction :type "/Game/Blueprints/Enums/EFactions Enum") (Health :type Integer) (Icon :type "Texture2D Object Reference"))
  (return (`self.Name`) (`self.Faction`) (`self.Health`) (`self.Icon`)))
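; Default unit puppet Blueprint that builds a unit's visual mesh and collision capsule size from its UNITStats data.
; The construction script previews the mesh on a debug component and sizes the capsule radius from the scaled mesh's Y bound plus padding.
; BeginPlay spawns the runtime mesh component using the stats' height, rotation and scale.
; Getter functions expose the assigned mesh and the child components under HardpointsRoot.
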(event `self.ReceiveBeginPlay`
  (bind (_unit_health _unit_mesh _unit_speed _unit_turn_rate _unit_accel _unit_faction _unit_patrol_radius _unit_sensor_range _unit_z_location _unit_engage_distance _unit_mesh_scale _debug_override_mesh_rotation) (break `/Game/Blueprints/Units/UnitStatsStruct` (`self.UNIT_Stats`)))
  (bind (_relativelocation_x _relativelocation_y) (`KismetMathLibrary.BreakVector` (`SceneComponent.RelativeLocation` (`self.Mesh_Root`))))
  (bind _returnvalue (`AddComponent|NODE_AddStaticMeshComponent-1` :`RelativeTransform` (`KismetMathLibrary.MakeTransform` (`KismetMathLibrary.MakeVector` _relativelocation_x _relativelocation_y _unit_z_location) _debug_override_mesh_rotation (`KismetMathLibrary.MakeVector` _unit_mesh_scale _unit_mesh_scale _unit_mesh_scale))))
  (bind _output_get (set `self.UNIT_Assigned_Mesh` _returnvalue))
  (`StaticMeshComponent.SetStaticMesh` _output_get _unit_mesh))

(fn `GetUnitHardpoints`
  (returns (Hardpoints :type "Array of SceneComponent Object Reference"))
  (return (`SceneComponent.GetChildrenComponents` (`self.Hardpoints_Root`) false)))

(fn `GetUnitMesh`
  (returns (`Unit Mesh` :type "StaticMesh Object Reference"))
  (return (`StaticMeshComponent.StaticMesh` (`self.UNIT_Assigned_Mesh`))))

(fn `UserConstructionScript`
  (bind (_unit_stats_unit_health _unit_stats_unit_mesh _unit_stats_unit_speed _unit_stats_unit_turn_rate _unit_stats_unit_accel _unit_stats_unit_faction _unit_stats_unit_patrol_radius _unit_stats_unit_sensor_range _unit_stats_unit_z_location _unit_stats_unit_engage_distance _unit_stats_unit_mesh_scale _unit_stats_debug_override_mesh_rotation) (break `/Game/Blueprints/Units/UnitStatsStruct` (`self.UNIT_Stats`)))
  (bind _debug_mesh_0 (`self.DEBUG_Mesh_0`))
  ;[1 0 0.8355] DEBUG - Make Chosen Mesh Visible in Viewport
  (`StaticMeshComponent.SetStaticMesh` _debug_mesh_0 _unit_stats_unit_mesh)
  (`SceneComponent.K2_SetWorldRotation` _debug_mesh_0 _unit_stats_debug_override_mesh_rotation false false)
  (`SceneComponent.SetWorldScale3D` _debug_mesh_0 (`KismetMathLibrary.MakeVector` _unit_stats_unit_mesh_scale _unit_stats_unit_mesh_scale _unit_stats_unit_mesh_scale))
  ;[1 1 1] Set Capsule Radius Based on Mesh
  (`CapsuleComponent.SetCapsuleRadius` (`self.Capsule`) (+ (* (.y (`.Max` (break `Box` (`StaticMesh.GetBoundingBox` _unit_stats_unit_mesh)))) _unit_stats_unit_mesh_scale) 30.0) true))
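; Base turret actor that turns to face an enemy and plays a muzzle flash when it is in range.
; While CanSeeEnemy is true, Tick smoothly interpolates the turret's yaw toward TargetVector; neither variable is set here.
; Inside EngageDistance, a Delay on Tick paces the muzzle emitter.
; No projectile or damage logic exists here, and the cannon sound node is unconnected.
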(event `self.ReceiveBeginPlay`)

(event `self.ReceiveTick`
  (params (DeltaSeconds :type "Float (single-precision)"))
  (bind _targetvector (`self.TargetVector`))
  (bind (_returnvalue_location _returnvalue_rotation) (`KismetMathLibrary.BreakTransform` (`SceneComponent.K2_GetComponentToWorld` (`self.Turret`))))
  (bind (_returnvalue_roll _returnvalue_pitch _returnvalue_yaw) (`KismetMathLibrary.BreakRotator` (`KismetMathLibrary.FindLookAtRotation` _returnvalue_location _targetvector)))
  (if (`self.CanSeeEnemy`)
    (`SceneComponent.K2_SetWorldRotation` (`self.Turret`) (`KismetMathLibrary.RInterpTo` _returnvalue_rotation (`KismetMathLibrary.MakeRotator` 0.0 0.0 _returnvalue_yaw) (`GameplayStatics.GetWorldDeltaSeconds`) 3.0) false false)
    (if (not (>= (`KismetMathLibrary.Vector_Distance` _returnvalue_location _targetvector) (`self.EngageDistance`)))
      (`KismetSystemLibrary.Delay` 2.0)
      (`GameplayStatics.SpawnEmitterAttached` "/Game/AdvancedTurnBasedTileToolkit/Maps/Advanced/FX/Particles/Abilities/Primary/FX/P_STD_MUZZLE.P_STD_MUZZLE" (`self.MuzzleScene`)))))

(fn `UserConstructionScript`)
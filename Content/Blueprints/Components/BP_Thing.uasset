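; BP_Thing is a turret that fires projectiles at an enemy assigned through the TargetedEnemy event, which also stores the instigating unit.
; While the target is valid, Tick smoothly turns the Turret toward it using only the look-at yaw.
; A Delay on Tick throttles fire to roughly once a second, spawning BP_Projectile at the turret with that instigator and playing a shot sound.
; GrabSelectedUnits is an empty stub.
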(event `/Game/Blueprints/Interfaces/Skirmish_Interface.Targeted Enemy`
  (params (Enemy :type "Actor Object Reference") (Instigator :type "/Game/Blueprints/Units/BP_Base_Unit Object Reference"))
  (set `self.Target` Enemy)
  (set `self.InstigatingUnit` Instigator))

(event `self.ReceiveTick`
  (params (DeltaSeconds :type "Float (single-precision)"))
  (bind _target (`self.Target`))
  (bind (_returnvalue_location _returnvalue_rotation) (`KismetMathLibrary.BreakTransform` (`SceneComponent.K2_GetComponentToWorld` (`self.Turret`))))
  (bind (_returnvalue_roll _returnvalue_pitch _returnvalue_yaw) (`KismetMathLibrary.BreakRotator` (`KismetMathLibrary.FindLookAtRotation` _returnvalue_location (`self.K2_GetActorLocation` _target))))
  (if (`KismetSystemLibrary.IsValid` _target)
    (`SceneComponent.K2_SetWorldRotation` (`self.Turret`) (`KismetMathLibrary.RInterpTo` _returnvalue_rotation (`KismetMathLibrary.MakeRotator` 0.0 0.0 _returnvalue_yaw) (`GameplayStatics.GetWorldDeltaSeconds`) 3.0) false false)
    (`KismetSystemLibrary.Delay` 1.0)
    (`|SpawnActorFromClass` "/Game/Blueprints/Components/BP_Projectile.BP_Projectile_C" (`SceneComponent.K2_GetComponentToWorld` (`self.Turret`)) "AlwaysSpawn" "OverrideRootScale" null (`self.InstigatingUnit`))
    (`GameplayStatics.PlaySoundAtLocation` "/Game/Sounds/Future_Weapons_2_-_Energy_Gun_-_shot_single_variation_05.Future_Weapons_2_-_Energy_Gun_-_shot_single_variation_05" (`self.K2_GetActorLocation`) (struct) 0.1 1.0 0.0 null null null null)))

(fn `GrabSelectedUnits`
  (returns (`Selected Units` :type "Array of Actor Object Reference"))
  (return))

(fn `UserConstructionScript`)
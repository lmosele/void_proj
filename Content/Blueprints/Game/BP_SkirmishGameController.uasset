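; Player controller for an RTS skirmish mode that handles marquee unit selection, move orders and the selected-units UI.
; Left mouse drives HUD marquee messages, with Tick updating while held via the misnamed IsRMBPressed flag.
; Right-click release sends HUD-selected units to the cursor hit, offset diagonally by index at fixed height.
; Selection events add unit widgets and toggle RTS camera following, noted as broken; its own GrabSelectedUnits is an empty stub.
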(event `/Game/Blueprints/Interfaces/Skirmish_Interface.SelectUnit`
  ;[1 1 1] Set camera based on selection event, doesnt work
  (bind _bp_openrtscamera (`/OpenRTSCamera/BPFL_RTSCameraSystem.Get OpenRTS Camera`))
  (`RTSCamera.UnFollowTarget` (`/OpenRTSCamera/BP_RTSCamera.RTSCamera` _bp_openrtscamera)))

(event `/Game/Blueprints/Interfaces/Skirmish_Interface.SelectSingleUnit`
  (params (Unit :type "Actor Object Reference"))
  ;[1 1 1] Set camera based on selection event, doesnt work
  (bind _bp_openrtscamera (`/OpenRTSCamera/BPFL_RTSCameraSystem.Get OpenRTS Camera`))
  (`RTSCamera.FollowTarget` (`/OpenRTSCamera/BP_RTSCamera.RTSCamera` _bp_openrtscamera) Unit))

(event `/Game/Blueprints/Interfaces/Skirmish_Interface.AddSelectedUnitToUI`
  (params (SelectedUnitWidget :type "UserWidget Object Reference"))
  (`HorizontalBox.AddChildToHorizontalBox` (`/Game/Blueprints/UI/WB_Skirmish_Selected_Units.UnitsBox` (`self.SelectedUnitsUI`)) SelectedUnitWidget))

(event `self.ReceiveBeginPlay`
  (`WidgetBlueprintLibrary.SetInputMode_GameAndUIEx` self null "LockAlways" false)
  (set `self.bShowMouseCursor` true)
  (bind _returnvalue (`|CreateWidget` "/Game/Blueprints/UI/WB_Skirmish_Selected_Units.WB_Skirmish_Selected_Units_C"))
  (bind _output_get (set `self.SelectedUnitsUI` _returnvalue))
  (`UserWidget.AddToViewport` _output_get 0))

(event `self.ReceiveTick`
  (params (DeltaSeconds :type "Float (single-precision)"))
  ;[1 1 1] Left Click to Marquee Select
  (if (`self.IsRMBPressed`)
    (message `/Game/Blueprints/Interfaces/Skirmish_Interface.MarqueeHeld` (`self.GetHUD`))))

(event `Key|LeftMouseButton`
  (params (Key :type "Key Structure"))
  (bind _returnvalue (`self.GetHUD`))
  (:`Pressed`
    ;[1 1 1] Left Click to Marquee Select
    (set `self.IsRMBPressed` true)
    (message `/Game/Blueprints/Interfaces/Skirmish_Interface.MarqueePressed` _returnvalue))
  (:`Released`
    (set `self.IsRMBPressed` false)
    (message `/Game/Blueprints/Interfaces/Skirmish_Interface.MarqueeReleased` _returnvalue)))

(event `Key|RightMouseButton`
  (params (Key :type "Key Structure"))
  (bind (_right_click_location_x _right_click_location_y) (`KismetMathLibrary.BreakVector` (`self.Right Click Location`)))
  (:`Released`
    ;[1 1 1] Right Click to Move Unit
    (set `self.Right Click Location` (`.Location` (`GameplayStatics.BreakHitResult` (`self.GetHitResultUnderCursorByChannel` "TraceTypeQuery1"))))
    (bind _selected_units (message `/Game/Blueprints/Interfaces/Skirmish_Interface.GrabSelectedUnits` (`self.GetHUD`)))
    (for (_array_element _array_index) _selected_units
      (bind _returnvalue (* _array_index 100))
      (message `/Game/Blueprints/Interfaces/Skirmish_Interface.UnitMoveCommand` _array_element (`KismetMathLibrary.MakeVector` (+ _returnvalue _right_click_location_x) (+ _returnvalue _right_click_location_y) 10.0)))))

(fn `GrabSelectedUnits`
  (returns (`Selected Units` :type "Array of Actor Object Reference"))
  (return))

(fn `UserConstructionScript`)
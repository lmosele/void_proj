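; Test AI pawn that patrols random reachable points and engages BP_Skirmish_Unit pawns spotted by PawnSensing.
; Tick drives AIMoveTo toward the patrol point or target, interpolating body rotation and widening the acceptance radius to half sensor range while tracking.
; With an enemy visible, the turret turns toward it and plays muzzle effects and sound within engage distance, without projectiles or damage.
; Debug cone, arrow, sphere and prints expose sensing, turning and destinations.
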(event `self.ReceiveBeginPlay`
  ;[1 1 1] Create Initial Patrol zIndex - Need to improve this
  (set `self.zIndex` (.z (`self.K2_GetActorLocation`)))
  (set `self.EngageDistance` 10.0)
  (set `self.SensorRange` 1000.0)
  (`self.SetPatrol`))

(event `self.ReceiveTick`
  (params (DeltaSeconds :type "Float (single-precision)"))
  (bind _targetvector (`self.TargetVector`))
  (bind _turret (`self.Turret`))
  (bind _projectilspawn (`self.ProjectilSpawn`))
  (bind _targetvector_2 (`self.TargetVector`))
  (bind _returnvalue (`SceneComponent.K2_GetComponentLocation` _turret))
  (`|ExecutionSequence`
    (:`then_0`
      (if (`self.CanSeeEnemy`)
        (set `self.DEBUGChaseColor` (`KismetMathLibrary.Conv_LinearColorToColor` (`KismetMathLibrary.LinearColor_Red`)))
        (else
          (set `self.DEBUGChaseColor` (`KismetMathLibrary.Conv_LinearColorToColor` (`KismetMathLibrary.LinearColor_Green`)))))
      (`KismetSystemLibrary.DrawDebugConeInDegrees` (`self.K2_GetActorLocation`) (`self.GetActorForwardVector`) (`self.SensorRange`) 180.0 0.0 12 (`KismetMathLibrary.Conv_ColorToLinearColor` (`self.DEBUGChaseColor`))))
    (:`then_1`
      (`self.newRotateTo` DeltaSeconds)
      (if (<= (.yaw (`KismetMathLibrary.FindLookAtRotation` (`self.GetActorForwardVector` self) _targetvector)) (.yaw (`self.K2_GetActorRotation` self)))
        (set `self.DEBUGFaceColor` (`KismetMathLibrary.Conv_LinearColorToColor` (`KismetMathLibrary.LinearColor_Green`)))
        (set `self.IsTurning` false)
        (set `self.CanMove` true)
        (else
          (set `self.DEBUGFaceColor` (`KismetMathLibrary.Conv_LinearColorToColor` (`KismetMathLibrary.LinearColor_Red`)))
          (set `self.IsTurning` true)
          (set `self.CanMove` false)))
      (`KismetSystemLibrary.DrawDebugArrow` (`self.K2_GetActorLocation` self) _targetvector 0.0 (`KismetMathLibrary.Conv_ColorToLinearColor` (`self.DEBUGFaceColor`))))
    (:`then_2`
      ;[1 1 1] Move To Location
      (`AITask_MoveTo.AIMoveTo` (`AIBlueprintHelperLibrary.GetAIController` self) (`self.TargetVector`) null (`self.EngageDistance`) "Enable" "Disable" true true (`self.CanMove`) "Disable"
        (:`OnMoveFinished`
          (`self.TargetUnit`
            (:`then`)
            (:`else`
              (`KismetSystemLibrary.Delay` 2.0)
              (`self.SetPatrol`))))))
    (:`then_3`
      ;[1 1 1] Keep Checking if Unit is Visible in Distance
      (`self.TargetUnit`
        (:`then`
          (if (`PawnSensingComponent.bSeePawns` (`self.PawnSensing`))
            (set `self.TargetVector` (`self.K2_GetActorLocation` (`self.TargetUnit`)))
            (set `self.CanSeeEnemy` true)
            (set `self.EngageDistance` (/ (`self.SensorRange`) 2.0))
            (else
              (set `self.CanSeeEnemy` false)
              (set `self.EngageDistance` 10.0)
              (set `self.TargetUnit` null))))
        (:`else`)))
    (:`then_4`
      (if (`self.CanSeeEnemy`)
        (`SceneComponent.K2_SetWorldRotation` (`self.Turret`) (`KismetMathLibrary.RInterpTo` (`SceneComponent.K2_GetComponentRotation` _turret) (`KismetMathLibrary.MakeRotator` 0.0 0.0 (.yaw (`KismetMathLibrary.FindLookAtRotation` _returnvalue _targetvector_2))) DeltaSeconds 3.0) false false)
        (if (not (>= (`KismetMathLibrary.Vector_Distance` _returnvalue _targetvector_2) (`self.EngageDistance`)))
          (`KismetSystemLibrary.Delay` 0.2)
          (`GameplayStatics.SpawnEmitterAttached` "/Game/AdvancedTurnBasedTileToolkit/Maps/Advanced/FX/Particles/Abilities/Primary/FX/P_STD_MUZZLE.P_STD_MUZZLE" _projectilspawn)
          (`GameplayStatics.SpawnSoundAttached` null _projectilspawn "None" (0.0 0.0 0.0) (struct) "KeepRelativeOffset" false 0.9 0.8 0.0 null null))))
    (:`then_5`
      (`KismetSystemLibrary.PrintString` (`KismetStringLibrary.Conv_DoubleToString` (`self.EngageDistance`))))))

(event `self.PawnSensing.OnSeePawn`
  (params (Pawn :type "Pawn Object Reference"))
  ;[1 1 1] Set Visbility
  (bind _asbp_skirmish_unit (cast `/Game/Blueprints/Units/BP_Skirmish_Unit` Pawn))
  (set `self.TargetUnit` _asbp_skirmish_unit)
  (bind _returnvalue (`self.K2_GetActorLocation` _asbp_skirmish_unit))
  (set `self.TargetVector` (`KismetMathLibrary.MakeVector` (.x _returnvalue) (.y _returnvalue)))
  (if (< (`KismetMathLibrary.Vector_Distance2D` (`self.K2_GetActorLocation`) _returnvalue) (`self.SensorRange`))
    (set `self.CanSeeEnemy` true)
    (else
      (set `self.CanSeeEnemy` false))))

(fn `newRotateTo`
  (params (DeltaTime :type "Float (single-precision)"))
  (if (not (`self.IsWithinDistance`))
    (`self.K2_SetActorRotation` (`KismetMathLibrary.RInterpTo` (`self.K2_GetActorRotation`) (`KismetMathLibrary.FindLookAtRotation` (`self.K2_GetActorLocation`) (`self.TargetVector`)) DeltaTime 0.7) true)))

(fn `SetPatrol`
  (if (`self.CanSeeEnemy`)
    _
    (else
      _))
  (bind _output_get (set `self.TargetVector` (`KismetMathLibrary.MakeVector` (.x (`NavigationSystemV1.K2_GetRandomReachablePointInRadius` (`self.K2_GetActorLocation`) (`self.PatrolRadius`) null null)) (.y (`NavigationSystemV1.K2_GetRandomReachablePointInRadius` (`self.K2_GetActorLocation`) (`self.PatrolRadius`) null null)) (`self.zIndex`))))
  (`KismetSystemLibrary.PrintString` (`KismetStringLibrary.Conv_VectorToString` _output_get))
  (`KismetSystemLibrary.DrawDebugSphere` _output_get 100.0 12 (struct :`R` 0.681644 :`G` 0.003043 :`B` 1.0 :`A` 1.0) 5.0 2.0)
  (return))

(fn `UserConstructionScript`)
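; BP_Traveler is a draft actor that hops between the nodes tracked by BP_NodeManager.
; On BeginPlay it finds the manager, flashes a debug sphere at the nearest node and snaps to that node's XY at a fixed height.
; Tick, throttled by a one-second Delay, asks the manager for the overlapped node and moves to its NodeNeighbor.
; The lerp alpha is 1, so each move is an instant jump.
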(event `self.ReceiveBeginPlay`
  (bind (_startpoint_x _startpoint_y) (`KismetMathLibrary.BreakVector` (`self.Startpoint`)))
  (bind _returnvalue (`GameplayStatics.GetActorOfClass` "/Game/Blueprints/Drafts/BP_NodeManager.BP_NodeManager_C"))
  (bind _returnvalue_2 (`self.K2_GetActorLocation` (`.ReturnValue` (`GameplayStatics.FindNearestActor` (`self.K2_GetActorLocation`) (`/Game/Blueprints/Drafts/BP_NodeManager.Node Actors` _returnvalue)))))
  (`KismetSystemLibrary.DrawDebugSphere` _returnvalue_2 100.0 12 (struct :`R` 0.660626 :`B` 1.0 :`A` 1.0) 1.0)
  (set `self.Startpoint` _returnvalue_2)
  (`self.K2_SetActorLocation` (`KismetMathLibrary.MakeVector` _startpoint_x _startpoint_y 100.0)))

(event `self.ReceiveTick`
  (params (DeltaSeconds :type "Float (single-precision)"))
  (`KismetSystemLibrary.Delay` 1.0)
  (bind _overlappednode (`/Game/Blueprints/Drafts/BP_NodeManager.GetOverlappedNode` (stale `self.ReceiveBeginPlay` _returnvalue)))
  (`self.K2_SetActorLocation` (`KismetMathLibrary.VLerp` (`self.K2_GetActorLocation`) (`self.K2_GetActorLocation` (`/Game/Blueprints/Drafts/BP_Node.NodeNeighbor` _overlappednode)) 1.0)))

(fn `UserConstructionScript`)
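; BP_Tile_Planet is a tile Blueprint that places a planet at its mesh location.
; On BeginPlay it spawns a scaled-down BP_Planet_1 at the static mesh's world location and adds that location to PlanetLocations.
; Every Tick it loops over PlanetLocations and spawns a new building-destruction particle emitter at each one, with no delay or condition.
; The construction script only calls the parent.
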(event `self.ReceiveBeginPlay`
  (bind _returnvalue (`SceneComponent.K2_GetComponentLocation` (`self.StaticMesh`)))
  (`|SpawnActorFromClass` "/Game/Planet_Creator_1/Blueprint/BP_Planet_1.BP_Planet_1_C" (`KismetMathLibrary.MakeTransform` _returnvalue (struct) (0.09 0.09 0.09)) "Undefined" "OverrideRootScale" null null)
  (`KismetArrayLibrary.Array_Add` (`self.PlanetLocations`) _returnvalue))

(event `self.ReceiveTick`
  (params (DeltaSeconds :type "Float (single-precision)"))
  (for _array_element (`self.PlanetLocations`)
    (`GameplayStatics.SpawnEmitterAtLocation` "/Game/Realistic_Starter_VFX_Pack_Vol2/Particles/Destruction/P_Destruction_Building_B.P_Destruction_Building_B" _array_element)))

(fn `UserConstructionScript`
  (`parent.UserConstructionScript`))
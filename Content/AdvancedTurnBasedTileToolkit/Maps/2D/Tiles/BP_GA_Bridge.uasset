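; BP_GA_Bridge is a 2D grid bridge tile that becomes passable once enough torches are lit.
; Each AttemptRaise call increments a lit-torch counter and compares it to the required count.
; On first reaching that count, a DoOnce tells the grid manager to make the bridge's tile passable and spawns a SetActorVisibility action actor targeting the bridge.
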(event `AttemptRaise`
  (bind _currenttorcheslit (`self.CurrentTorchesLit`))
  (`/Engine/EditorBlueprintResources/StandardMacros.IncrementInt` _currenttorcheslit
    (:`  `
      (if (>= _currenttorcheslit (`self.RequiredTorchesLit`))
        (`/Engine/EditorBlueprintResources/StandardMacros.DoOnce` false
          (:`Completed`
            (`/Game/AdvancedTurnBasedTileToolkit/Core/Grid/BP_GridManager.MakeTilePassable` (`self.GridManagerRef`) (`self.GridIndex`) 1)
            (`|SpawnActorFromClass` "/Game/AdvancedTurnBasedTileToolkit/Core/Actions/BP_Action_SetActorVisibility.BP_Action_SetActorVisibility_C" (`KismetMathLibrary.MakeTransform` (0.0 0.0 0.0)) "AlwaysSpawn" "OverrideRootScale" null self false -1.0 "NewEnumerator0" null)))))))

(fn `UserConstructionScript`
  (`parent.UserConstructionScript`))
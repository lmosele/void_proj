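; Hydra attack ability for the 2D stats units in the turn-based tile toolkit, striking a target tile once per head.
; The head count comes from the owning Hydra unit, falling back to one if the cast fails.
; Each strike spawns an attack action, subtracts the Damage stat from the target's health, then spawns a short delay action.
; The grid is rechecked before every strike, so attacks stop once the tile holds no unit.
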(fn `ExecuteAbility`
  (params (TargetIndexIn :type Integer))
  (returns (bSuccess :type Boolean))
  (locals (LocalHeads :type Integer :default 0))
  (bind _asbp_unit_stats_2d_hydra (cast `/Game/AdvancedTurnBasedTileToolkit/Maps/2D/Units/BP_Unit_Stats_2D_Hydra` (`self.OwningUnit`))
    (:`then`
      (set `local.LocalHeads` (`/Game/AdvancedTurnBasedTileToolkit/Maps/2D/Units/BP_Unit_Stats_2D_Hydra.Heads` _asbp_unit_stats_2d_hydra)))
    (:`CastFailed`
      (set `local.LocalHeads` 1)))
  (for _ (range 1 (+ (`local.LocalHeads`) 1))
    (if (`BlueprintMapLibrary.Map_Contains` (`/Game/AdvancedTurnBasedTileToolkit/Core/Grid/BP_GridManager.GridUnits` (`self.GridManagerRef`)) (`local.TargetIndexIn`))
      (bind _unitdata (message `/Game/AdvancedTurnBasedTileToolkit/Maps/StrategyRpg/Core/BPI_StatsUnit.GetUnitData` (`self.OwningUnit`)))
      (`|SpawnActorFromClass` "/Game/AdvancedTurnBasedTileToolkit/Maps/2D/Actions/BP_Action_Attack_Hydra.BP_Action_Attack_Hydra_C" (`KismetMathLibrary.MakeTransform` (0.0 0.0 0.0)) "AlwaysSpawn" "OverrideRootScale" null (`/Game/AdvancedTurnBasedTileToolkit/Core/Units/BP_Unit.Puppet` (`self.OwningUnit`)) (`/Game/AdvancedTurnBasedTileToolkit/Core/Units/BP_Unit.Puppet` (`BlueprintMapLibrary.Map_Find` (`/Game/AdvancedTurnBasedTileToolkit/Core/Grid/BP_GridManager.GridUnits` (`self.GridManagerRef`)) (`local.TargetIndexIn`))) _unitdata (`self.OwningUnit`) -1.0 "NewEnumerator0" null)
      (bind (_bhasstat _value) (message `/Game/AdvancedTurnBasedTileToolkit/Maps/Experimental/StatSystem/Core/BPI_Stats.GetStatValue` (`self.OwningActor`) (struct :`TagName` "Stat.Damage")))
      (`/Game/AdvancedTurnBasedTileToolkit/Core/Units/BP_Unit.ModifyHealth` (`BlueprintMapLibrary.Map_Find` (`/Game/AdvancedTurnBasedTileToolkit/Core/Grid/BP_GridManager.GridUnits` (`self.GridManagerRef`)) (`local.TargetIndexIn`)) (* _value -1.0) true 0.2)
      (`|SpawnActorFromClass` "/Game/AdvancedTurnBasedTileToolkit/Core/Actions/BP_Action_Delay.BP_Action_Delay_C" (`KismetMathLibrary.MakeTransform` (0.0 0.0 0.0)) "AlwaysSpawn" "OverrideRootScale" null 0.3 "NewEnumerator0" null)
      (else
        (return true))))
  (return true))

(fn `UserConstructionScript`
  (`parent.UserConstructionScript`))
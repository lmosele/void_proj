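; BP_Status_Poisoned is a strategy RPG status effect that damages the unit it is attached to, evidently once per turn.
; On server setup it binds itself to the owner's dispatcher hub for the turn-end event.
; When run, it reads a stat value from the owning unit and subtracts it from that unit's health with auto animation and a short end delay.
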(event `self.ServerSetupStatus`
  (`/Game/AdvancedTurnBasedTileToolkit/Maps/Experimental/StatSystem/Core/BP_DispatcherHubComponent.BindEventToHub` (`self.GetOwnersDispatcherHub`) self (struct :`TagName` "Event.TurnEnd")))

(event `/Game/AdvancedTurnBasedTileToolkit/Maps/Experimental/StatSystem/Core/BPI_EventHolder.RunEvent`
  (params (EventTag :type "GameplayTag Structure") (CallingObject :type "Object Object Reference (by ref)") (bGlobal :type Boolean) (Payload :type "Object Object Reference (by ref)"))
  (bind _asbp_unit (cast `/Game/AdvancedTurnBasedTileToolkit/Core/Units/BP_Unit` (`self.GetOwner`)))
  (bind (_bhasstat _value) (message `/Game/AdvancedTurnBasedTileToolkit/Maps/Experimental/StatSystem/Core/BPI_Stats.GetStatValue` (`self.GetOwner`) (`self.Stat`)))
  (`/Game/AdvancedTurnBasedTileToolkit/Core/Units/BP_Unit.ModifyHealth` _asbp_unit (* _value -1.0) true 0.5))
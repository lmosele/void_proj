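; Venomous status for the strategy RPG example that makes the owning unit's attacks apply Poisoned stacks.
; On server setup it binds to the owner's post-attack event.
; When that event runs, it adds Poisoned to the attack payload's stat message, scaled by the owner's Stack value times the status value, each clamped to at least one.
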(event `self.ServerSetupStatus`
  (`self.BindToLocalEventsFromOwner` (struct :`GameplayTags` (struct :`(TagName` "Event.UnitAttackingPost")))))

(event `/Game/AdvancedTurnBasedTileToolkit/Maps/Experimental/StatSystem/Core/BPI_EventHolder.RunEvent`
  (params (EventTag :type "GameplayTag Structure") (CallingObject :type "Object Object Reference (by ref)") (bGlobal :type Boolean) (Payload :type "Object Object Reference (by ref)"))
  (`|SwitchGameplayTag` EventTag
    (:`Event.UnitAttackingPost`
      (if (`KismetSystemLibrary.IsValid` Payload)
        (bind (_bhasstat _value) (message `/Game/AdvancedTurnBasedTileToolkit/Maps/Experimental/StatSystem/Core/BPI_Stats.GetStatValue` (`self.GetOwner`) (struct :`TagName` "Stat.Stack")))
        (message `/Game/AdvancedTurnBasedTileToolkit/Maps/Experimental/StatSystem/Core/BPI_Stats.AddToStat` Payload (struct :`TagName` "Stat.Status.Poisoned") (* (`KismetMathLibrary.FMax` _value 1.0) (`KismetMathLibrary.FMax` (`self.StatValue`) 1.0)))))))
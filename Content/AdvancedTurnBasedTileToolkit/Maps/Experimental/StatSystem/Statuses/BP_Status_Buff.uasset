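; BP_Status_Buff is a status Blueprint in the turn-based tile toolkit's experimental stat system, representing a buff to stats.
; When its value changes, it scans the gameplay tags in its stat data for ones matching the Stat tag, including child tags.
; For each match it sends the owner a stat message carrying the difference between new and old value, then runs the parent handler.
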(fn `RunOnStatusModified`
  (params (NewValue :type "Float (double-precision)") (OldValue :type "Float (double-precision)"))
  (for _array_element (`BlueprintGameplayTagLibrary.BreakGameplayTagContainer` (`.GameplayTags_13_0FBFCF8E4FAB22E862B30FB5F4874198` (break `/Game/AdvancedTurnBasedTileToolkit/Maps/Experimental/StatSystem/Core/FStat` (`self.StatData`))))
    (if (`BlueprintGameplayTagLibrary.MatchesTag` _array_element (struct :`TagName` "Stat"))
      (message `/Game/AdvancedTurnBasedTileToolkit/Maps/Experimental/StatSystem/Core/BPI_Stats.AddToStat` (`self.GetOwner`) _array_element (- (`local.NewValue`) (`local.OldValue`)))))
  (`parent.RunOnStatusModified` (`local.NewValue`) (`local.OldValue`)))
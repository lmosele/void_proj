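; BP_StatusComponent is a base component for one status effect in the turn-based toolkit's stat system.
; It writes its value into the owner's stats component and fires a stat event on each change.
; When the value is not positive and the stat's removal setting allows it, it clears its stat and status entries and destroys itself.
; Helpers bind events to the owner's dispatcher hub, while setup, name and priority are empty defaults.
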(event `ServerSetupStatus`)

(event `self.ReceiveBeginPlay`
  (`self.ServerSetupStatus`))

(fn `BindToLocalEventsFromOwner`
  (params (Events :type "GameplayTagContainer Structure"))
  (`/Game/AdvancedTurnBasedTileToolkit/Maps/Experimental/StatSystem/Core/BP_DispatcherHubComponent.BindMultipleEventsToHub` (`Actor.GetComponentByClass` (`self.GetOwner`) "/Game/AdvancedTurnBasedTileToolkit/Maps/Experimental/StatSystem/Core/BP_DispatcherHubComponent.BP_DispatcherHubComponent_C") self Events)
  (return))

(fn `GetFriendlyName`
  (returns (FriendlyName :type Text))
  (return ""))

(fn `GetOwnersDispatcherHub`
  (returns (ReturnValue :type "/Game/AdvancedTurnBasedTileToolkit/Maps/Experimental/StatSystem/Core/BP_DispatcherHubComponent Object Reference"))
  (return (`Actor.GetComponentByClass` (`self.GetOwner`) "/Game/AdvancedTurnBasedTileToolkit/Maps/Experimental/StatSystem/Core/BP_DispatcherHubComponent.BP_DispatcherHubComponent_C")))

(fn `GetPriority`
  (returns (Priority :type "Float (double-precision)"))
  (return 0.0))

(fn `GetStatValue`
  (returns (bHasStat :type Boolean) (StatValue :type "Float (double-precision)"))
  (bind (_value _returnvalue) (`BlueprintMapLibrary.Map_Find` (`/Game/AdvancedTurnBasedTileToolkit/Maps/Experimental/StatSystem/Core/BP_StatsComponent.Stats` (`self.OwnersStatsComponent`)) (`self.Stat`)))
  (if _returnvalue
    (return true _value)
    (else
      (return false 0.0))))

(fn `RemoveStatus`
  (params (OldValue :type "Float (double-precision)"))
  (locals (LocalZeroValue :type "Float (double-precision)" :default 0.0))
  (`BlueprintMapLibrary.Map_Remove` (`/Game/AdvancedTurnBasedTileToolkit/Maps/Experimental/StatSystem/Core/BP_StatsComponent.Stats` (`self.OwnersStatsComponent`)) (`self.Stat`))
  (`BlueprintMapLibrary.Map_Remove` (`/Game/AdvancedTurnBasedTileToolkit/Maps/Experimental/StatSystem/Core/BP_StatsComponent.Statuses` (`self.OwnersStatsComponent`)) (`self.Stat`))
  (`/Game/AdvancedTurnBasedTileToolkit/Maps/Experimental/StatSystem/Core/BP_StatsComponent.CallStatEvent` (`self.OwnersStatsComponent`) (`self.Stat`) (`local.OldValue`) (`local.LocalZeroValue`) false)
  (`self.K2_DestroyComponent`)
  (return))

(fn `RunOnStatusCreated`
  (params (StatusValue :type "Float (double-precision)"))
  (`self.RunOnStatusModified` StatusValue)
  (return))

(fn `RunOnStatusModified`
  (params (NewValue :type "Float (double-precision)") (OldValue :type "Float (double-precision)"))
  (if (or (> NewValue 0.0) (`|EnumInequality` (`.StatRemoval_28_6211D6E94E5C5AE767B8DA8AD2B3660D` (break `/Game/AdvancedTurnBasedTileToolkit/Maps/Experimental/StatSystem/Core/FStat` (`self.StatData`))) "NewEnumerator1"))
    (`BlueprintMapLibrary.Map_Add` (`/Game/AdvancedTurnBasedTileToolkit/Maps/Experimental/StatSystem/Core/BP_StatsComponent.Stats` (`self.OwnersStatsComponent`)) (`self.Stat`) NewValue)
    (set `self.StatValue` (`local.NewValue`))
    (`/Game/AdvancedTurnBasedTileToolkit/Maps/Experimental/StatSystem/Core/BP_StatsComponent.CallStatEvent` (`self.OwnersStatsComponent`) (`self.Stat`) (`local.OldValue`) (`local.NewValue`) false)
    (return)
    (else
      (`self.RemoveStatus` OldValue)
      (return))))
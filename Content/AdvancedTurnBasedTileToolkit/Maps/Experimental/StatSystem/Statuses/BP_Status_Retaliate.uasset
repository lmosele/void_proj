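; Retaliate status for the turn-based tile toolkit that makes the owning unit counterattack when it is attacked.
; On the owner's local post-attack event, it checks that the owner is not the active actor and the attacker is one tile away, diagonals included.
; It then spawns a delay action and calls DefaultAttack on the attacker.
; StatValue caps retaliations, with the counter reset by the global turn-start event.
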(event `self.ServerSetupStatus`
  (bind _asbp_unit_stats (cast `/Game/AdvancedTurnBasedTileToolkit/Maps/Experimental/StatSystem/Units/BP_Unit_Stats` (`self.GetOwner`)))
  (set `self.OwningUnit` _asbp_unit_stats)
  (`self.BindToLocalEventsFromOwner` (struct :`GameplayTags` (struct :`(TagName` "Event.UnitAttackedPost"))))
  (`/Game/AdvancedTurnBasedTileToolkit/Maps/Experimental/StatSystem/Core/BPFL_DispatcherHub.BindEventToGlobalDispatcherHub` self (struct :`TagName` "Event.TurnStart")))

(event `/Game/AdvancedTurnBasedTileToolkit/Maps/Experimental/StatSystem/Core/BPI_EventHolder.RunEvent`
  (params (EventTag :type "GameplayTag Structure") (CallingObject :type "Object Object Reference (by ref)") (bGlobal :type Boolean) (Payload :type "Object Object Reference (by ref)") (CallTags :type "GameplayTagContainer Structure (by ref)"))
  (`|SwitchGameplayTag` EventTag
    (:`Event.UnitAttackedPost`
      (if bGlobal
        _
        (elif (> (`self.StatValue`) (`KismetMathLibrary.Conv_IntToDouble` (`self.UsesThisTurn`)))
          (if (!= (`/Game/AdvancedTurnBasedTileToolkit/Core/BP_TurnManager.ActiveActor` (`.TurnManager` (`/Game/AdvancedTurnBasedTileToolkit/Core/BPFL_Singletons.GetTurnManager`))) (`self.GetOwner`))
            (bind _asbp_unit_stats (cast `/Game/AdvancedTurnBasedTileToolkit/Maps/Experimental/StatSystem/Units/BP_Unit_Stats` CallingObject))
            (if (== (`/Game/AdvancedTurnBasedTileToolkit/Core/Grid/BP_GridManager.FindDistanceIinTilesBetweenIndexes` (`.GridManager` (`/Game/AdvancedTurnBasedTileToolkit/Core/BPFL_Singletons.GetGridManager`)) (`/Game/AdvancedTurnBasedTileToolkit/Core/Units/BP_Unit.GridIndex` _asbp_unit_stats) (`/Game/AdvancedTurnBasedTileToolkit/Core/Units/BP_Unit.GridIndex` (`self.OwningUnit`)) false) 1)
              (`|SpawnActorFromClass` "/Game/AdvancedTurnBasedTileToolkit/Core/Actions/BP_Action_Delay.BP_Action_Delay_C" (`KismetMathLibrary.MakeTransform` (0.0 0.0 0.0)) "Undefined" "OverrideRootScale" null (`self.RetaliationDelay`) "NewEnumerator0" null)
              (`/Engine/EditorBlueprintResources/StandardMacros.IncrementInt` (`self.UsesThisTurn`)
                (:`  `
                  (`/Game/AdvancedTurnBasedTileToolkit/Core/Units/BP_Unit.DefaultAttack` (`self.OwningUnit`) _asbp_unit_stats))))))))
    (:`Event.TurnStart`
      (set `self.UsesThisTurn` 0))))
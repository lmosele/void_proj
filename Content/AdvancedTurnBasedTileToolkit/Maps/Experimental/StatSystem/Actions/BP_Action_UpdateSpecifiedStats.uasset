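; Turn-based toolkit action that pushes selected stat values from a Unit to the stats component of its Puppet.
; Setup snapshots each tagged stat from the Unit's BP_StatsComponent into a map, defaulting missing ones to zero.
; In networked games the map is also flattened into StatsArray, from which non-server machines rebuild it on play.
; Playing the action applies the map to the Puppet's BP_StatsComponent and ends immediately.
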(event `self.SetupAction`
  (bind _unit (`self.Unit`))
  (bind _stattags_gameplaytags (break `GameplayTagContainer` (`self.StatTags`)))
  (bind _puppet (message `/Game/AdvancedTurnBasedTileToolkit/Core/BPI_Initiative.GetPuppet` _unit))
  (set `self.Puppet` _puppet)
  (for _array_element _stattags_gameplaytags
    (bind (_value _returnvalue) (`BlueprintMapLibrary.Map_Find` (`/Game/AdvancedTurnBasedTileToolkit/Maps/Experimental/StatSystem/Core/BP_StatsComponent.Stats` (`self.GetComponentByClass` _unit "/Game/AdvancedTurnBasedTileToolkit/Maps/Experimental/StatSystem/Core/BP_StatsComponent.BP_StatsComponent_C")) _array_element))
    (if _returnvalue
      (`BlueprintMapLibrary.Map_Add` (`self.SpecifiedStats`) _array_element _value)
      (else
        (`BlueprintMapLibrary.Map_Add` (`self.SpecifiedStats`) _array_element))))
  (if (not (`KismetSystemLibrary.IsStandalone`))
    (bind _keys (`BlueprintMapLibrary.Map_Keys` (`self.SpecifiedStats`)))
    (for _array_element_2 _keys
      (`KismetArrayLibrary.Array_Add` (`self.StatsArray`) (make `/Game/AdvancedTurnBasedTileToolkit/Maps/Experimental/StatSystem/Core/FStatValue` _array_element_2 (`BlueprintMapLibrary.Map_Find` (`self.SpecifiedStats`) _array_element_2))))))

(event `self.PlayAction`
  (if (not (`KismetSystemLibrary.IsServer`))
    (for _array_element (`self.StatsArray`)
      (`BlueprintMapLibrary.Map_Add` (`self.SpecifiedStats`) (break `/Game/AdvancedTurnBasedTileToolkit/Maps/Experimental/StatSystem/Core/FStatValue` _array_element) (`.Value_5_123A91854F29D970C997DB92A40F5ECF` (break `/Game/AdvancedTurnBasedTileToolkit/Maps/Experimental/StatSystem/Core/FStatValue` _array_element)))))
  (`/Game/AdvancedTurnBasedTileToolkit/Maps/Experimental/StatSystem/Core/BP_StatsComponent.UpdateSpecifiedStats` (`self.GetComponentByClass` (`self.Puppet`) "/Game/AdvancedTurnBasedTileToolkit/Maps/Experimental/StatSystem/Core/BP_StatsComponent.BP_StatsComponent_C") (`self.SpecifiedStats`))
  (`self.EndAction` true))

(fn `UserConstructionScript`
  (`parent.UserConstructionScript`))
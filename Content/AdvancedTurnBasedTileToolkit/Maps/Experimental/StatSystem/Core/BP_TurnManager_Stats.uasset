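; Turn manager variant for the experimental stat system that broadcasts turn start and end as tagged events through dispatcher hubs.
; BeginNewTurn fires Event.TurnStart on the global hub before running the parent logic.
; BeginNextValidActorTurn first sends Event.TurnEnd to the active unit's hub component, or to the global hub when no unit is valid, then defers to the parent.
; Other overrides only call their parent.
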(event `self.BeginNewTurn`
  (`/Game/AdvancedTurnBasedTileToolkit/Maps/Experimental/StatSystem/Core/BPFL_DispatcherHub.CallEventInGlobalDispatcherHub` (struct :`TagName` "Event.TurnStart") self)
  (`parent.BeginNewTurn`))

(event `self.ResumeAfterOngoingActionsDone`
  (`parent.ResumeAfterOngoingActionsDone`))

(event `self.BeginNextValidActorTurn`
  (params (bUseCustomDelay :type Boolean) (CustomDelay :type "Float (single-precision)"))
  (`|ExecutionSequence`
    (:`then_0`
      (bind _activeunit (`self.ActiveUnit`)
        (:`then`
          (`/Game/AdvancedTurnBasedTileToolkit/Maps/Experimental/StatSystem/Core/BP_DispatcherHubComponent.CallEvent` (`self.GetComponentByClass` _activeunit "/Game/AdvancedTurnBasedTileToolkit/Maps/Experimental/StatSystem/Core/BP_DispatcherHubComponent.BP_DispatcherHubComponent_C") (struct :`TagName` "Event.TurnEnd") (`self.ActiveUnit`) null true))
        (:`else`
          (`/Game/AdvancedTurnBasedTileToolkit/Maps/Experimental/StatSystem/Core/BPFL_DispatcherHub.CallEventInGlobalDispatcherHub` (struct :`TagName` "Event.TurnEnd") self))))
    (:`then_1`
      (`parent.BeginNextValidActorTurn` bUseCustomDelay CustomDelay))))

(fn `UserConstructionScript`
  (`parent.UserConstructionScript`))
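; BP_StatPayload is a data object describing a single stat change in the toolkit's experimental stat system.
; One update function stores the stat, its old and new values, a pre-change flag and the stat data.
; Getters expose these values and the computed delta, and helper checks report whether the stat rose from zero or below to positive, or now sits at zero or below.
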(fn `GetPayloadNewStatValue`
  (returns (StatValue :type "Float (double-precision)"))
  (return (`self.NewValue`)))

(fn `GetPayloadOldStatValue`
  (returns (StatValue :type "Float (double-precision)"))
  (return (`self.OldValue`)))

(fn `GetPayloadStat`
  (returns (Stat :type "GameplayTag Structure"))
  (return (`self.Stat`)))

(fn `GetPayloadStatChange`
  (returns (StatChange :type "Float (double-precision)"))
  (return (- (`self.NewValue`) (`self.OldValue`))))

(fn `GetPayloadStatData`
  (returns (StatData :type "/Game/AdvancedTurnBasedTileToolkit/Maps/Experimental/StatSystem/Core/FStat Structure"))
  (return (`self.StatData`)))

(fn `IsPayloadNewStat`
  (returns (bIsNew :type Boolean))
  (return (and (<= (`self.OldValue`) 0.0) (> (`self.NewValue`) 0.0))))

(fn `IsPayloadStatZero`
  (returns (bIsZero :type Boolean))
  (return (<= (`self.NewValue`) 0.0)))

(fn `UpdateStatPayload`
  (params (Stat :type "GameplayTag Structure (by ref)") (OldValue :type "Float (double-precision) (by ref)") (NewValue :type "Float (double-precision) (by ref)") (bCalledPreChange :type Boolean) (StatData :type "/Game/AdvancedTurnBasedTileToolkit/Maps/Experimental/StatSystem/Core/FStat Structure (by ref)"))
  (set `self.Stat` Stat)
  (set `self.OldValue` OldValue)
  (set `self.NewValue` NewValue)
  (set `self.bCalledPreChange` bCalledPreChange)
  (set `self.StatData` StatData)
  (return))
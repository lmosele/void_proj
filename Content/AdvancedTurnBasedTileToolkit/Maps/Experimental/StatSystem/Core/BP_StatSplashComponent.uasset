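; Component that pops up floating splash text when its owner's stats change, as part of the tile toolkit's experimental stat system.
; On BeginPlay it binds to the owner's dispatcher hub for the configured stat tags, then reacts to nonzero change payloads.
; Health and Stack show absolute amounts, while other stats append the rounded change to their name, all in the stat's color.
; Texts spawn as BP_TextSplash actors, queued and spaced by a delay.
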(event `self.ReceiveBeginPlay`
  (`/Game/AdvancedTurnBasedTileToolkit/Maps/Experimental/StatSystem/Core/BP_DispatcherHubComponent.BindMultipleEventsToHub` (`Actor.GetComponentByClass` (`self.GetOwner`) "/Game/AdvancedTurnBasedTileToolkit/Maps/Experimental/StatSystem/Core/BP_DispatcherHubComponent.BP_DispatcherHubComponent_C") self (`self.StatsToShow`)))

(event `/Game/AdvancedTurnBasedTileToolkit/Maps/Experimental/StatSystem/Core/BPI_EventHolder.RunEvent`
  (params (EventTag :type "GameplayTag Structure") (CallingObject :type "Object Object Reference (by ref)") (bGlobal :type Boolean) (Payload :type "Object Object Reference (by ref)"))
  (bind _statchange (message `/Game/AdvancedTurnBasedTileToolkit/Maps/Experimental/StatSystem/Core/BPI_StatPayload.GetPayloadStatChange` Payload))
  (if (!= _statchange 0.0)
    (bind _stat (message `/Game/AdvancedTurnBasedTileToolkit/Maps/Experimental/StatSystem/Core/BPI_StatPayload.GetPayloadStat` Payload))
    (`|SwitchGameplayTag` _stat
      (:`Default`
        (bind _statdata (message `/Game/AdvancedTurnBasedTileToolkit/Maps/Experimental/StatSystem/Core/BPI_StatPayload.GetPayloadStatData` Payload))
        (bind ((`FriendlyName_17_36FDE9024396FE9345596E9FB8C90F56` _friendlyname) (`Color_43_872105E848DD18BCB7BA80A51EE9B27D` _color)) (break `/Game/AdvancedTurnBasedTileToolkit/Maps/Experimental/StatSystem/Core/FStat` _statdata))
        (`self.DisplaySplashText` (`KismetTextLibrary.Conv_StringToText` (`KismetStringLibrary.Concat_StrStr` (`KismetTextLibrary.Conv_TextToString` _friendlyname) " " (`KismetStringLibrary.Conv_IntToString` (`KismetMathLibrary.Round` _statchange)))) (`KismetMathLibrary.Conv_ColorToLinearColor` _color)))
      (:`Stat.Health`
        (bind _statdata_2 (message `/Game/AdvancedTurnBasedTileToolkit/Maps/Experimental/StatSystem/Core/BPI_StatPayload.GetPayloadStatData` Payload :!label _label))
        (`self.DisplaySplashText` (`KismetTextLibrary.Conv_DoubleToText` (`KismetMathLibrary.Abs` _statchange) "HalfToEven") (`KismetMathLibrary.Conv_ColorToLinearColor` (`.Color_43_872105E848DD18BCB7BA80A51EE9B27D` (break `/Game/AdvancedTurnBasedTileToolkit/Maps/Experimental/StatSystem/Core/FStat` _statdata_2)))))
      (:`Stat.Stack`
        (goto _label)))))

(event `DisplaySplashText`
  (params (DisplayText :type Text) (Color :type "LinearColor Structure" :default (struct :`R` 1.0 :`G` 1.0 :`B` 1.0 :`A` 1.0)))
  (bind (_output_text _output_color) (break `/Game/AdvancedTurnBasedTileToolkit/Maps/Experimental/StatSystem/Core/FColoredText` (`|GetArrayItem` (`self.QueuedText`))))
  (if (`self.bReady`)
    (`|SpawnActorFromClass` "/Game/AdvancedTurnBasedTileToolkit/Maps/Experimental/StatSystem/Core/BP_TextSplash.BP_TextSplash_C" (`self.K2_GetComponentToWorld`) "AlwaysSpawn" "OverrideRootScale" null DisplayText (`KismetMathLibrary.Conv_LinearColorToColor` Color) null)
    (set `self.bReady` false)
    (`KismetSystemLibrary.Delay` (`self.DelayBetweenText`))
    (set `self.bReady` true)
    (if (> (`KismetArrayLibrary.Array_Length` (`self.QueuedText`)) 0)
      (`self.DisplaySplashText` _output_text (`KismetMathLibrary.Conv_ColorToLinearColor` _output_color))
      (`KismetArrayLibrary.Array_Remove` (`self.QueuedText`)))
    (else
      (`KismetArrayLibrary.Array_Add` (`self.QueuedText`) (make `/Game/AdvancedTurnBasedTileToolkit/Maps/Experimental/StatSystem/Core/FColoredText` DisplayText (`KismetMathLibrary.Conv_LinearColorToColor` Color))))))

(fn `GetFriendlyName`
  (returns (FriendlyName :type Text))
  (return ""))

(fn `GetPriority`
  (returns (Priority :type "Float (double-precision)"))
  (return 0.0))
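; BP_IconSplash is a short-lived actor in the experimental stat system that flashes an icon in the world.
; The construction script creates a dynamic material instance on IconMesh, which BeginPlay fills with the Icon texture and Color.
; The TL_Buff timeline then drives the mesh scale and material opacity, and the actor destroys itself when it finishes.
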(event `self.ReceiveBeginPlay`
  (`MaterialInstanceDynamic.SetTextureParameterValue` (`self.IconMaterial`) "Texture" (`self.Icon`))
  (`MaterialInstanceDynamic.SetVectorParameterValue` (`self.IconMaterial`) "Color" (`self.Color`))
  (bind (_direction _scale _opacity) (`Timeline|TL_Buff` :!via `PlayFromStart`)
    (:`Update`
      (`SceneComponent.SetRelativeScale3D` (`self.IconMesh`) (`KismetMathLibrary.Conv_DoubleToVector` _scale))
      (`MaterialInstanceDynamic.SetScalarParameterValue` (`self.IconMaterial`) "Opacity" _opacity))
    (:`Finished`
      (`self.K2_DestroyActor`))))

(fn `UserConstructionScript`
  (bind _returnvalue (`PrimitiveComponent.CreateDynamicMaterialInstance` (`self.IconMesh`) 0 null "None"))
  (set `self.IconMaterial` _returnvalue))
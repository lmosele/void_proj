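; Overwatch status effect for the turn-based tile toolkit that makes its owning unit take a reaction shot at a moving enemy.
; On activation it listens for units entering tiles during simulation, filtering for living, non-allied units within range and line of sight.
; The first valid target triggers a hard-coded Laser Rifle ability, then queues camera follow and a delay.
; The effect unbinds and disables after that shot or when its turn-start event runs.
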(event `self.Activate`
  (params (`Target Unit` :type "/Game/AdvancedTurnBasedTileToolkit/Core/Units/BP_Unit Object Reference"))
  (`parent.Activate` `Target Unit`)
  (add `/Game/AdvancedTurnBasedTileToolkit/Core/Grid/BP_GridManager.OnUnitEnterTileSimulate` (`self.GridManagerRef`) (delegate `CheckOverwatch`)))

(event `CheckOverwatch`
  (params (Unit :type "/Game/AdvancedTurnBasedTileToolkit/Core/Units/BP_Unit Object Reference") (GridIndex :type Integer))
  (bind _gridmanagerref (`self.GridManagerRef`))
  (bind _gridindex (`/Game/AdvancedTurnBasedTileToolkit/Core/Units/BP_Unit.GridIndex` (`self.OwningUnit`)))
  (bind _gridindex_2 (`/Game/AdvancedTurnBasedTileToolkit/Core/Units/BP_Unit.GridIndex` (`self.TargetUnit`)))
  (bind _distance (`/Game/AdvancedTurnBasedTileToolkit/Core/Grid/BP_GridManager.FindDistanceIinTilesBetweenIndexes` _gridmanagerref _gridindex _gridindex_2 false))
  (set `self.TargetUnit` Unit)
  (bind _targetunit (`self.TargetUnit`)
    (:`then`
      (if (not (`BlueprintSetLibrary.Set_Contains` (`/Game/AdvancedTurnBasedTileToolkit/Core/Units/BP_Unit.AlliedFactions` (`self.OwningUnit`)) (`/Game/AdvancedTurnBasedTileToolkit/Core/Units/BP_Unit.Faction` _targetunit)))
        (if (< _distance (`self.Range`))
          (bind _bvisible (`/Game/AdvancedTurnBasedTileToolkit/Core/Grid/BP_GridManager.CheckIfTileIsVisibleFromOtherTile` (`self.GridManagerRef`) _gridindex _gridindex_2 (* _distance (`/Game/AdvancedTurnBasedTileToolkit/Core/Grid/BP_GridManager.TileXSize` _gridmanagerref)) true))
          (if _bvisible
            (if (> (`/Game/AdvancedTurnBasedTileToolkit/Core/Units/BP_Unit.CurrentHealth` (`self.TargetUnit`)) 0.0)
              (`|ExecutionSequence`
                (:`then_0`
                  (remove `/Game/AdvancedTurnBasedTileToolkit/Core/Grid/BP_GridManager.OnUnitEnterTileSimulate` (`self.GridManagerRef`) (delegate `CheckOverwatch`))
                  (bind (_bspawnednew _abilityref) (message `/Game/AdvancedTurnBasedTileToolkit/Core/BPI_PC.GetOrAddAbility` (`.PlayerControllerATBTT` (`/Game/AdvancedTurnBasedTileToolkit/Core/BPFL_Singletons.GetPlayerControllerATBTT`)) "/Game/AdvancedTurnBasedTileToolkit/Maps/Advanced/Abilities/BP_Ability_LaserRifle.BP_Ability_LaserRifle_C"))
                  (bind _asbp_ability_laser_rifle (cast `/Game/AdvancedTurnBasedTileToolkit/Maps/Advanced/Abilities/BP_Ability_LaserRifle` _abilityref))
                  (set `/Game/AdvancedTurnBasedTileToolkit/Core/Abilities/BP_Ability.OwningUnit` (`self.OwningUnit`) _asbp_ability_laser_rifle)
                  (`/Game/AdvancedTurnBasedTileToolkit/Core/Abilities/BP_Ability.ExecuteAbility` _asbp_ability_laser_rifle (`/Game/AdvancedTurnBasedTileToolkit/Core/Units/BP_Unit.GridIndex` (`self.TargetUnit`)))
                  (bind _targetunit_2 (`self.TargetUnit`)
                    (:`then`
                      (`/Game/AdvancedTurnBasedTileToolkit/Core/BP_GridCamera.QueueFollowActor` (`.GridCamera` (`/Game/AdvancedTurnBasedTileToolkit/Core/BPFL_Singletons.GetGridCamera`)) (`/Game/AdvancedTurnBasedTileToolkit/Core/Units/BP_Unit.Puppet` _targetunit_2))
                      (`/Game/AdvancedTurnBasedTileToolkit/Core/BP_ActionManager.QueueDelay` (`.ActionManager` (`/Game/AdvancedTurnBasedTileToolkit/Core/BPFL_Singletons.GetActionManager`)) 1.0))
                    (:`else`)))
                (:`then_1`
                  (`self.Disable`))))))))
    (:`else`)))

(event `self.RunOnTurnStart`
  (remove `/Game/AdvancedTurnBasedTileToolkit/Core/Grid/BP_GridManager.OnUnitEnterTileSimulate` (`self.GridManagerRef`) (delegate `CheckOverwatch`))
  (`self.Disable`))

(fn `UserConstructionScript`
  (`parent.UserConstructionScript`))
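; BP_Event_Test is a test actor for the global event dispatcher hub.
; On BeginPlay it binds itself as the event holder for the Interact.EnterTile gameplay tag.
; When RunEvent fires, it prints the tag name and multiplies its scale by (2, 0, 0), doubling X and zeroing Y and Z.
; Its GetFriendlyName and GetPriority functions return empty and zero defaults.
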(event `self.ReceiveBeginPlay`
  (`/Game/AdvancedTurnBasedTileToolkit/Maps/Experimental/StatSystem/Core/BPFL_DispatcherHub.BindEventToGlobalDispatcherHub` self (struct :`TagName` "Interact.EnterTile")))

(event `/Game/AdvancedTurnBasedTileToolkit/Maps/Experimental/StatSystem/Core/BPI_EventHolder.RunEvent`
  (params (EventTag :type "GameplayTag Structure") (CallingObject :type "Object Object Reference (by ref)") (bGlobal :type Boolean) (Payload :type "Object Object Reference (by ref)"))
  (`KismetSystemLibrary.PrintString` (`KismetStringLibrary.Conv_NameToString` (`BlueprintGameplayTagLibrary.GetTagName` EventTag)))
  (`self.SetActorScale3D` (* (`self.GetActorScale3D`) (2.0 0.0 0.0))))

(fn `GetFriendlyName`
  (returns (FriendlyName :type Text))
  (return ""))

(fn `GetPriority`
  (returns (Priority :type "Float (double-precision)"))
  (return 0.0))

(fn `UserConstructionScript`)
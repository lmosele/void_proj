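; Configurable procedural planet actor with a surface mesh and two atmosphere shells, styled through exposed variables.
; Its construction script creates dynamic material instances for all three, then pushes parameters for atmosphere, clouds, continents, poles, equator, oceans, lava and textures.
; With a valid LightSource, it feeds that actor's forward vector into atmosphere lighting and sunset orientation, scales the shells by AtmosphereHeight and clears RefreshMaterial.
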(fn `UserConstructionScript`
  (bind _atmosphere_1_material (`self.Atmosphere_1_Material`))
  (bind _planet_material (`self.Planet_Material`))
  (bind _planet_material_2 (`self.Planet_Material`))
  (bind _atmosphere_2_material (`self.Atmosphere_2_Material`))
  (bind _atmosphere_falloff (`self.Atmosphere_Falloff`))
  (bind _planet_material_3 (`self.Planet_Material`))
  (bind _planet_material_4 (`self.Planet_Material`))
  (bind _atmosphere_falloff_2 (`self.Atmosphere_Falloff`))
  (bind _planet_material_5 (`self.Planet_Material`))
  (bind _light_source (`self.Light Source`))
  (bind _atmosphere_color (`self.Atmosphere Color`))
  (bind _planet_material_6 (`self.Planet_Material`))
  (bind _planet_material_7 (`self.Planet_Material`))
  (bind _returnvalue (`KismetMathLibrary.Conv_RotatorToVector` (`self.K2_GetActorRotation` _light_source)))
  (bind _returnvalue_2 (+ (`SceneComponent.K2_GetComponentScale` (`self.Planet`)) (`self.Atmosphere_Height`)))
  (bind _returnvalue_3 (`KismetMathLibrary.Conv_VectorToLinearColor` _returnvalue))
  (bind _returnvalue_4 (`PrimitiveComponent.CreateDynamicMaterialInstance` (`self.Atmosphere_2`) 0 (`self.Material_Instance_Atmosphere`) "None"))
  (set `self.Atmosphere_2_Material` _returnvalue_4)
  (bind _returnvalue_5 (`PrimitiveComponent.CreateDynamicMaterialInstance` (`self.Atmosphere_1`) 0 (`self.Material_Instance_Atmosphere`) "None"))
  (set `self.Atmosphere_1_Material` _returnvalue_5)
  (bind _returnvalue_6 (`PrimitiveComponent.CreateDynamicMaterialInstance` (`self.Planet`) 0 (`self.Material_Instance_Planet`) "None"))
  (set `self.Planet_Material` _returnvalue_6)
  (`|ExecutionSequence`
    (:`then_0`
      (`MaterialInstanceDynamic.SetScalarParameterValue` (`self.Atmosphere_1_Material`) "Atmosphere_Brightness" (`self.Atmosphere_Brightness`))
      (`MaterialInstanceDynamic.SetScalarParameterValue` _planet_material "Atmosphere_Intensity" (`self.Inner Atmosphere_Intensity`))
      (`MaterialInstanceDynamic.SetScalarParameterValue` _planet_material "Clouds_Opacity" (`self.Clouds Opacity`))
      (`MaterialInstanceDynamic.SetScalarParameterValue` _planet_material "Clouds_Turbolence" (`self.Clouds Turbolence`))
      (`MaterialInstanceDynamic.SetVectorParameterValue` _planet_material "Clouds_Color" (`self.Clouds Color`))
      (`MaterialInstanceDynamic.SetVectorParameterValue` _planet_material "Atmosphere_Color" _atmosphere_color)
      (`MaterialInstanceDynamic.SetVectorParameterValue` (`self.Atmosphere_1_Material`) "Atmosphere_Color" _atmosphere_color)
      (`MaterialInstanceDynamic.SetScalarParameterValue` _planet_material_6 "Extinction_Intensity" (`self.Extinction Intensity`))
      (`MaterialInstanceDynamic.SetVectorParameterValue` _planet_material_6 "Color_Extinction" (`self.Extinction Color`))
      (`MaterialInstanceDynamic.SetScalarParameterValue` _planet_material_6 "Greenhouse" (`self.Greenhouse Effect`))
      (`MaterialInstanceDynamic.SetScalarParameterValue` _atmosphere_2_material "Atmosphere_Brightness" (`self.Atmosphere_Brightness`))
      (`MaterialInstanceDynamic.SetVectorParameterValue` _atmosphere_2_material "Atmosphere_Color" (`self.Atmosphere Color`))
      (`MaterialInstanceDynamic.SetScalarParameterValue` (`self.Atmosphere_1_Material`) "InnerFalloff" _atmosphere_falloff_2)
      (`MaterialInstanceDynamic.SetScalarParameterValue` (`self.Atmosphere_2_Material`) "InnerFalloff" _atmosphere_falloff_2)
      (`MaterialInstanceDynamic.SetScalarParameterValue` (`self.Planet_Material`) "Clouds_Speed" (`self.Clouds Speed`))
      (`MaterialInstanceDynamic.SetScalarParameterValue` (`self.Planet_Material`) "Clouds_Normal" (`self.Clouds Normal`)))
    (:`then_1`
      (`MaterialInstanceDynamic.SetScalarParameterValue` _planet_material_3 "Continent_1_Altitude" (`self.Continent 1 Altitude`))
      (`MaterialInstanceDynamic.SetScalarParameterValue` _planet_material_3 "Erosion_Continent_1" (`self.Erosion Continent 1`))
      (`MaterialInstanceDynamic.SetScalarParameterValue` _planet_material_3 "Continent_1_Style" (`self.Continent 1 Style`))
      (`MaterialInstanceDynamic.SetScalarParameterValue` _planet_material_3 "Continent_2_Altitude" (`self.Continent 2 Altitude`))
      (`MaterialInstanceDynamic.SetScalarParameterValue` _planet_material_3 "Continent_2_Style" (`self.Continent 2 Style`))
      (`MaterialInstanceDynamic.SetScalarParameterValue` _planet_material_3 "Continents_Spikiness" (`self.Continents_Spikiness`))
      (`MaterialInstanceDynamic.SetScalarParameterValue` _planet_material_3 "Erosion_Continent_2" (`self.Erosion Continent 2`))
      (`MaterialInstanceDynamic.SetScalarParameterValue` _planet_material_3 "Normal_Intensity" (`self.Normal Intensity`))
      (`MaterialInstanceDynamic.SetScalarParameterValue` _planet_material_3 "Surface_Warp" (`self.Continents Warp`))
      (`MaterialInstanceDynamic.SetVectorParameterValue` _planet_material_3 "Color_1" (`self.Color_1`))
      (`MaterialInstanceDynamic.SetVectorParameterValue` _planet_material_3 "Color_2" (`self.Color_2`)))
    (:`then_2`
      (`MaterialInstanceDynamic.SetScalarParameterValue` _planet_material_4 "Poles_Altitude" (`self.Poles Altitude`))
      (`MaterialInstanceDynamic.SetScalarParameterValue` _planet_material_4 "Equator_Altitude" (`self.Equator Altitude`))
      (`MaterialInstanceDynamic.SetScalarParameterValue` _planet_material_4 "Equator_Sharpness" (`self.Equator Sharpness`))
      (`MaterialInstanceDynamic.SetScalarParameterValue` _planet_material_4 "Poles_Sharpness" (`self.Poles Sharpness`))
      (`MaterialInstanceDynamic.SetVectorParameterValue` _planet_material_4 "Color_Equator" (`self.Equator Color`))
      (`MaterialInstanceDynamic.SetVectorParameterValue` _planet_material_4 "Color_Poles" (`self.Poles Color`)))
    (:`then_3`
      (`MaterialInstanceDynamic.SetScalarParameterValue` _planet_material_5 "Sea_Level" (`self.Oceans Level`))
      (`MaterialInstanceDynamic.SetScalarParameterValue` _planet_material_5 "Snow_Level" (`self.Snow Level`))
      (`MaterialInstanceDynamic.SetScalarParameterValue` _planet_material_5 "Coast_Width" (`self.Coast Width`))
      (`MaterialInstanceDynamic.SetScalarParameterValue` _planet_material_5 "Poles_Ice" (`self.Poles Ice`))
      (`MaterialInstanceDynamic.SetVectorParameterValue` _planet_material_5 "Sea_Color" (`self.Sea Color`))
      (`MaterialInstanceDynamic.SetVectorParameterValue` _planet_material_5 "Coast_Color" (`self.Coast Color`)))
    (:`then_4`
      (`MaterialInstanceDynamic.SetScalarParameterValue` _planet_material_2 "Color_Contrast" (`self.Color Contrast`))
      (`MaterialInstanceDynamic.SetScalarParameterValue` _planet_material_2 "Diffuse_Intensity" (`self.Diffuse Intensity`))
      (`MaterialInstanceDynamic.SetTextureParameterValue` _planet_material_2 "Continent_1_A" (`self.Continent 1 A`))
      (`MaterialInstanceDynamic.SetTextureParameterValue` _planet_material_2 "Continent_1_B" (`self.Continent 1 B`))
      (`MaterialInstanceDynamic.SetTextureParameterValue` _planet_material_2 "Continent_2_A" (`self.Continent 2 A`))
      (`MaterialInstanceDynamic.SetTextureParameterValue` _planet_material_2 "Continent_2_B" (`self.Continent 2 B`))
      (`MaterialInstanceDynamic.SetTextureParameterValue` _planet_material_2 "Continent_Map" (`self.Continent Main Map`))
      (`MaterialInstanceDynamic.SetTextureParameterValue` _planet_material_2 "Diffuse_1" (`self.Diffuse 1`))
      (`MaterialInstanceDynamic.SetTextureParameterValue` _planet_material_2 "Diffuse_2" (`self.Diffuse 2`))
      (`MaterialInstanceDynamic.SetTextureParameterValue` _planet_material_2 "Cloud_Map" (`self.Cloud Map`)))
    (:`then_5`
      (`MaterialInstanceDynamic.SetScalarParameterValue` _planet_material_7 "Lava_Depth" (`self.Lava Depth`))
      (`MaterialInstanceDynamic.SetScalarParameterValue` _planet_material_7 "Lava_Intensity" (`self.Lava Intensity`))
      (`MaterialInstanceDynamic.SetScalarParameterValue` _planet_material_7 "Heat_Power" (`self.Heat Power`))
      (`MaterialInstanceDynamic.SetScalarParameterValue` _planet_material_7 "Heat_Intensity" (`self.Heat Intensity`))
      (`MaterialInstanceDynamic.SetVectorParameterValue` _planet_material_7 "Lava_Color_1" (`self.Lava Color 1`))
      (`MaterialInstanceDynamic.SetVectorParameterValue` _planet_material_7 "Lava_Color_2" (`self.Lava Color 2`)))
    (:`then_6`
      (`/Engine/EditorBlueprintResources/StandardMacros.IsValid` _light_source
        (:`Is Valid`
          (`MaterialInstanceDynamic.SetVectorParameterValue` (`self.Atmosphere_1_Material`) "LightDirection" _returnvalue_3)
          (`MaterialInstanceDynamic.SetVectorParameterValue` (`self.Atmosphere_2_Material`) "LightDirection" (`KismetMathLibrary.Conv_VectorToLinearColor` _returnvalue))
          (`MaterialInstanceDynamic.SetVectorParameterValue` (`self.Planet_Material`) "SunsetOrientation" _returnvalue_3)
          (`SceneComponent.SetWorldScale3D` (`self.Atmosphere_1`) _returnvalue_2)
          (`SceneComponent.SetWorldScale3D` (`self.Atmosphere_2`) _returnvalue_2)
          (if (< _atmosphere_falloff 0.0)
            (`MaterialInstanceDynamic.SetScalarParameterValue` _atmosphere_1_material "BrightSide_Size" (* _atmosphere_falloff -1.0))
            (else
              (`MaterialInstanceDynamic.SetScalarParameterValue` _atmosphere_1_material "BrightSide_Size" _atmosphere_falloff)))
          (set `self.Refresh material` false))))))
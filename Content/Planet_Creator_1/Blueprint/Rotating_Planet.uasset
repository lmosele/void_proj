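; Rotating planet actor that slowly turns and shows distant explosions attached at random points.
; Tick eases the planet's world rotation toward a fixed target with RInterpTo, so it is not a continuous spin.
; A Delay on Tick throttles spawning of the Explosion_Far Niagara system to about once per second on one of six scene components.
; The random index's upper bound equals the array length, so it can fall out of range.
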(event `self.ReceiveBeginPlay`)

(event `self.ReceiveTick`
  (params (DeltaSeconds :type "Float (single-precision)"))
  (bind _array (`|MakeArray` (`self.Scene`) (`self.Scene1`) (`self.Scene2`) (`self.Scene3`) (`self.Scene4`) (`self.Scene5`)))
  (`SceneComponent.K2_SetWorldRotation` (`self.Planet`) (`KismetMathLibrary.RInterpTo` (`SceneComponent.K2_GetComponentRotation` (`self.Planet`)) (struct :`Pitch` 10.0 :`Yaw` 270.0) DeltaSeconds 0.02) false false)
  (`KismetSystemLibrary.Delay` 1.0)
  (`NiagaraFunctionLibrary.SpawnSystemAttached` "/Game/Particles/Explosion_Far.Explosion_Far" (`|GetArrayItem` _array (`KismetMathLibrary.RandomIntegerInRange` 0 (`KismetArrayLibrary.Array_Length` _array))) "None" (0.0 0.0 0.0) (struct) "KeepRelativeOffset"))

(fn `UserConstructionScript`
  (`parent.UserConstructionScript`))